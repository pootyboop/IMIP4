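; BP_EnemySpawn is an effect actor, apparently an enemy spawn marker, made of two spinning static meshes with a lifetime counted in beats.
; On BeginPlay it binds to a rhythm event, and each beat decrements Lifetime until the actor destroys itself at zero.
; Tick rotates the meshes around yaw in opposite directions, using Speed scaled by world delta time.
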(event `self.ReceiveBeginPlay`
  (`/Game/Blueprints/BPFL_BlueprintFunctionLibrary.bindEventToRhythm` "NewEnumerator1" (delegate `OnBeat`)))

(event `OnBeat`
  (bind _result (`/Engine/EditorBlueprintResources/StandardMacros.DecrementInt` (`self.lifetime`))
    (:`  `
      (if (<= _result 0)
        (`self.K2_DestroyActor`)))))

(event `self.ReceiveTick`
  (params (DeltaSeconds :type "Float (single-precision)"))
  (bind _returnvalue (* (`self.speed`) (`GameplayStatics.GetWorldDeltaSeconds`)))
  (`SceneComponent.K2_AddRelativeRotation` (`self.StaticMesh`) (`KismetMathLibrary.MakeRotator` 0.0 0.0 _returnvalue) false false)
  (`SceneComponent.K2_AddRelativeRotation` (`self.StaticMesh1`) (`KismetMathLibrary.MakeRotator` 0.0 0.0 (* _returnvalue -1.0)) false false))

(fn `UserConstructionScript`)