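; BP_Plutocrat is an enemy Blueprint that can spawn a force field as its special ability.
; Each beat calls the parent, plays the idle animation and counts down the special cooldown, re-allowing the special when it reaches zero.
; When the special starts, it blocks further specials, resets the cooldown, plays the shield animation and spawns a BP_ForceField at its own location.
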(event `self.OnBeat`
  (`parent.OnBeat`)
  (`self.setAnim` "/Game/Meshes/Enemies/Plutocrat/Plutocrat_Anim_Armature_Idle.Plutocrat_Anim_Armature_Idle")
  (if (!= (`self.currSpecialCooldown`) 0)
    (bind _result (`/Engine/EditorBlueprintResources/StandardMacros.DecrementInt` (`self.currSpecialCooldown`))
      (:`  `
        (if (== _result 0)
          (set `self.isSpecialAllowed` true))))))

(event `self.SpecialStart`
  (`parent.SpecialStart`)
  (set `self.isSpecialAllowed` false)
  (set `self.currSpecialCooldown` (`self.specialCooldown`))
  (`self.setAnim` "/Game/Meshes/Enemies/Plutocrat/Plutocrat_Anim_Armature_Shield.Plutocrat_Anim_Armature_Shield")
  (`|SpawnActorFromClass` "/Game/Blueprints/Enemies/_EnemyTypes/BP_ForceField.BP_ForceField_C" (`KismetMathLibrary.Conv_VectorToTransform` (`self.K2_GetActorLocation`)) "Undefined" "MultiplyWithRoot" null null))

(fn `UserConstructionScript`
  (`parent.UserConstructionScript`))