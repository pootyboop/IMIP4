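; Butcher enemy that throws knives at the player's last remembered location.
; BeginPlay spawns a BP_ButcherKnife in each hand socket, and EndPlay destroys any still held.
; Inherited attack phase events drive it: face the player on preattack and tell, throw on attack, refill empty hands on recovery.
; Throwing prefers the right knife, falls back to the left, then clears that reference.
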(event `self.ReceiveBeginPlay`
  (`parent.ReceiveBeginPlay`)
  (`self.getNewKnives`)
  (add `self.OnEndPlay` (delegate `OnEndPlayEvent`)))

(event `OnEndPlayEvent` :!signature `self.OnEndPlay`
  (params (Actor :type "Actor Object Reference") (EndPlayReason :type "EEndPlayReason Enum" :default "Destroyed"))
  (bind _knifel (`self.knifeL`)
    (:`then`
      (`self.K2_DestroyActor` _knifel))
    (:`else`
      _))
  (bind _knifer (`self.knifeR`)
    (:`then`
      (`self.K2_DestroyActor` _knifer))
    (:`else`)))

(event `self.OnAttackPreattack`
  (`self.facePlayer` false :!label _label))

(event `self.OnAttackTell`
  (goto _label))

(event `self.OnAttackAttack`
  (`self.throw`))

(event `self.OnAttackRecovery`
  (`self.getNewKnives`))

(fn `getNewKnives`
  (`self.spawnKnife` false)
  (`self.spawnKnife` true))

(fn `spawnKnife`
  (params (isRight :type Boolean))
  (locals (newKnife :type "/Game/Blueprints/Enemies/Actions/Attack/BP_ButcherKnife Object Reference"))
  (bind _newknife (`local.newKnife`))
  (`/Engine/EditorBlueprintResources/StandardMacros.IsValid` (select `bool` isRight :`false` (`self.knifeL`) :`true` (`self.knifeR`))
    (:`Is Not Valid`
      (bind _returnvalue (`|SpawnActorFromClass` "/Game/Blueprints/Enemies/Actions/Attack/BP_ButcherKnife.BP_ButcherKnife_C" (`KismetMathLibrary.MakeTransform` (`self.K2_GetActorLocation`)) "Undefined" "MultiplyWithRoot" self null))
      (bind _output_get (set `local.newKnife` _returnvalue))
      (`self.K2_AttachToComponent` _output_get (`self.EnemySkeletalMesh`) (select `bool` (`local.isRight`) :`false` "hand_L" :`true` "hand_R" :!type "Name") "SnapToTarget" "SnapToTarget" "KeepWorld" true)
      (if (`local.isRight`)
        (set `self.knifeR` _newknife)
        (else
          (set `self.knifeL` _newknife))))))

(fn `throw`
  (locals (knifeToThrow :type "/Game/Blueprints/Enemies/Actions/Attack/BP_ButcherKnife Object Reference"))
  (bind _output_get (set `local.knifeToThrow` (select `bool` (`KismetSystemLibrary.IsValid` (`self.knifeR`)) :`false` (`self.knifeL`) :`true` (`self.knifeR`))))
  (`/Game/Blueprints/Enemies/Actions/Attack/BP_Projectile.throw` _output_get (`KismetMathLibrary.Conv_RotatorToVector` (`KismetMathLibrary.FindLookAtRotation` (`self.K2_GetActorLocation` _output_get) (`self.lastRememberedPlayerLocation`))) (`self.throwDist`) "NewEnumerator5")
  (if (`KismetSystemLibrary.IsValid` (`self.knifeR`))
    (set `self.knifeR` null)
    (else
      (set `self.knifeL` null))))

(fn `UserConstructionScript`
  (`parent.UserConstructionScript`))