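; BP_Bishop is an enemy type that attacks by firing a beam from the electricity on its head.
; The construction script snaps HeadElectricity to the skeletal mesh's Electricity socket, and that component's world location becomes the beam origin.
; Attack tell and preattack both call FacePlayer, then the attack fires at the last remembered player location.
; Startup and construction also run the parent enemy's logic.
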(event `self.ReceiveBeginPlay`
  (`parent.ReceiveBeginPlay`))

(event `self.OnAttackTell`
  (`self.facePlayer` false :!label _label))

(event `self.OnAttackPreattack`
  (goto _label))

(event `self.OnAttackAttack`
  (`self.fireBeam` (`SceneComponent.K2_GetComponentLocation` (`self.HeadElectricity`)) (`self.lastRememberedPlayerLocation`) 3000.0 (`/Game/Blueprints/Enemies/BPC_EnemyAI.printDebugInformation` (`self.BPC_EnemyAI`))))

(fn `setupElectricity`
  (`SceneComponent.K2_AttachToComponent` (`self.HeadElectricity`) (`self.EnemySkeletalMesh`) "Electricity" "SnapToTarget" "SnapToTarget" "KeepWorld" true))

(fn `UserConstructionScript`
  (`parent.UserConstructionScript`)
  (`self.setupElectricity`))