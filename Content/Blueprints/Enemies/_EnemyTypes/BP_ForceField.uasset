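; BP_ForceField is a temporary force field actor, filed under enemy types, whose lifetime is counted in rhythm beats.
; On BeginPlay it binds OnBeat to the rhythm system, and each beat decrements Lifetime until the actor destroys itself at zero.
; Tick slowly spins two sphere components around yaw in opposite directions, scaled by delta time.
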(event `self.ReceiveBeginPlay`
  (`/Game/Blueprints/BPFL_BlueprintFunctionLibrary.bindEventToRhythm` "NewEnumerator1" (delegate `OnBeat`)))

(event `OnBeat`
  (bind _result (`/Engine/EditorBlueprintResources/StandardMacros.DecrementInt` (`self.lifetime`))
    (:`  `
      (if (== _result 0)
        (`self.K2_DestroyActor`)))))

(event `self.ReceiveTick`
  (params (DeltaSeconds :type "Float (single-precision)"))
  (bind _returnvalue (* (`GameplayStatics.GetWorldDeltaSeconds`) 10.0))
  (`SceneComponent.K2_AddLocalRotation` (`self.Sphere`) (`KismetMathLibrary.MakeRotator` 0.0 0.0 _returnvalue) false false)
  (`SceneComponent.K2_AddLocalRotation` (`self.Sphere1`) (`KismetMathLibrary.MakeRotator` 0.0 0.0 (* _returnvalue -1.0)) false false))

(fn `UserConstructionScript`)