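; Squid enemy Blueprint that attacks by jumping up and lunging at the player.
; It overrides the inherited attack-phase events, each calling a movement or facing helper.
; Preattack jumps to a set height, and the tell turns it toward the player.
; The attack lunges to a set distance from the player with radius damage, then recovery faces the player again.
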(event `self.OnAttackPreattack`
  (`self.jumpToHeight` (`self.jumpHeight`)))

(event `self.OnAttackTell`
  (`self.facePlayer` true))

(event `self.OnAttackAttack`
  (`self.moveSetDistanceFromPlayer` (`self.lungeLandDistFromPlayer`) false (`self.lungeDamageRadius`) 2))

(event `self.OnAttackRecovery`
  (`self.facePlayer` false))

(fn `UserConstructionScript`
  (`parent.UserConstructionScript`))