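; BP_Hammer is a beat-driven hammer enemy that charges the player with a short-range area attack.
; It faces the player during preattack and tell, then moves to a set distance from them and deals radius damage.
; Between attacks, each beat alternates two running animations and checks player distance.
; Once the player is within first-attack range, it permanently unlocks attacking; the radius overlap events are unused.
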(event `self.ReceiveBeginPlay`
  (`parent.ReceiveBeginPlay`)
  (set `self.player` (`/Game/Blueprints/Enemies/BP_AIHivemind.player` (`/Game/Blueprints/BPFL_BlueprintFunctionLibrary.getAIHivemind`))))

(event `self.OnAttackPreattack`
  (`self.facePlayer` false :!label _label))

(event `self.OnAttackTell`
  (goto _label))

(event `self.OnAttackAttack`
  (`self.moveSetDistanceFromPlayer` 100.0 false 200.0 1))

(event `self.OnAttackRecovery`)

(event `self.AttackPlayerRadius.OnComponentBeginOverlap`
  (params (OverlappedComponent :type "PrimitiveComponent Object Reference") (OtherActor :type "Actor Object Reference") (OtherComp :type "PrimitiveComponent Object Reference") (OtherBodyIndex :type Integer) (bFromSweep :type Boolean) (SweepResult :type "HitResult Structure (by ref)"))
  ;[1 1 1] Won't attack until close to player. Once close to player at least once, will permanently be able to attack player from any range.
)

(event `self.AttackPlayerRadius.OnComponentEndOverlap`
  (params (OverlappedComponent :type "PrimitiveComponent Object Reference") (OtherActor :type "Actor Object Reference") (OtherComp :type "PrimitiveComponent Object Reference") (OtherBodyIndex :type Integer))
  ;[1 1 1] Won't attack until close to player. Once close to player at least once, will permanently be able to attack player from any range.
)

(event `self.OnBeat`
  (`parent.OnBeat`)
  (if (not (`self.isAttacking`))
    (`|ExecutionSequence`
      (:`then_0`
        (`/Engine/EditorBlueprintResources/StandardMacros.FlipFlop`
          (:`A`
            (bind _output_get (set `self.idleAnim` "/Game/Meshes/Enemies/Hammer/Hammer_Anim_Armature_Running1.Hammer_Anim_Armature_Running1"))
            (`self.setAnim` _output_get))
          (:`B`
            (bind _output_get_2 (set `self.idleAnim` "/Game/Meshes/Enemies/Hammer/Hammer_Anim_Armature_Running2.Hammer_Anim_Armature_Running2"))
            (`self.setAnim` _output_get_2))))
      (:`then_1`
        (if (and (not (`self.uniqueAttackCriteriaMet`)) (< (`KismetMathLibrary.Vector_Distance` (`self.K2_GetActorLocation` (`self.player`)) (`self.K2_GetActorLocation`)) (`self.firstAttackRange`)))
          (set `self.uniqueAttackCriteriaMet` true))))))

(fn `UserConstructionScript`
  (`parent.UserConstructionScript`))