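; Base enemy for a beat-driven VR game, with empty beat, move and attack events as override hooks.
; Attacks step through AttackInfo beats (tell, pre-attack, attack, recovery), setting animations and snapshotting the player's position at pre-attack.
; Movement helpers use BPC_EnemyAI points to snap or timeline-lerp with a Niagara trail, the lerp ending in radius damage.
; Also provides beam firing, defeat-type hints, and death that notifies spawner and hivemind.
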(event `self.ReceiveBeginPlay`
  (`parent.ReceiveBeginPlay`)
  (`self.setAnim` (`self.idleAnim`))
  (`self.spawnAlign`))

(event `OnBeat`)

(event `MoveStart`)

(event `AttackStart`)

(event `OnAttackTell`)

(event `OnAttackPreattack`)

(event `OnAttackAttack`)

(event `OnAttackRecovery`)

(event `LerpToSpot`
  (params (targetLocation :type "Vector Structure") (damagePlayerRadius :type "Float (double-precision)") (damageToDeal :type Integer) (instakill :type Boolean))
  (bind (_direction _alpha) (`Timeline|LerpMove` :!via `PlayFromStart`)
    (:`Update`
      (`self.K2_SetActorLocationAndRotation` (`KismetMathLibrary.VLerp` (`self.previousLocation`) targetLocation _alpha) (`self.solveBestRotation` true) true)
      (`self.updateLineRendererPositionPt2`))
    (:`Finished`
      (`self.damageAllWithinDistance` damagePlayerRadius damageToDeal instakill))))

(event `self.OnDestroyedKilled`
  (`parent.OnDestroyedKilled`)
  (bind _spawner (`self.spawner`)
    (:`then`
      (`/Game/Blueprints/Enemies/Waves/BP_EnemyWaveSpawner.enemyKilled` _spawner (`self.type`)))
    (:`else`
      _))
  (`self.deathFX`)
  (`/Game/Blueprints/Enemies/BPC_EnemyAI.removeFromHivemind` (`self.BPC_EnemyAI`))
  (`self.K2_DestroyActor`))

(fn `attackBeatTypeEffects`
  (params (attackBeatType :type "/Game/Blueprints/Enemies/Actions/Attack/EAttackBeatType Enum" :default "NewEnumerator0"))
  (switch `/Game/Blueprints/Enemies/Actions/Attack/EAttackBeatType` attackBeatType
    (:`NewEnumerator0`
      (`self.OnAttackTell`))
    (:`NewEnumerator1`
      (`self.updateLastRememberedPlayerPosition` (`self.attackCameraNotPlayerRoot`))
      (`self.OnAttackPreattack`)
      (`/Game/Blueprints/BPFL_BlueprintFunctionLibrary.tryPlayTrackByCondition` "NewEnumerator9" false true)
      (`self.spawnPreattackFX`))
    (:`NewEnumerator2`
      (`self.OnAttackAttack`))
    (:`NewEnumerator3`
      (`self.OnAttackRecovery`))))

(fn `damageAllWithinDistance`
  (params (radius :type "Float (double-precision)" :default 100.0) (damageToDeal :type Integer :default 1) (instakill :type Boolean))
  (bind _outactors (`KismetSystemLibrary.SphereOverlapActors` (`self.K2_GetActorLocation`) radius (`|MakeArray` "ObjectTypeQuery3" "ObjectTypeQuery2" :!type "EObjectTypeQuery Enum") "/Game/VRTemplate/Blueprints/VRPawn.VRPawn_C" (`|MakeArray` self :!type "Actor Object Reference")))
  (message `/Game/Blueprints/Interactive/Destroyable/BPI_Destroyable.Damage` (`|GetArrayItem` _outactors) (`local.damageToDeal`) (`local.instakill`) "NewEnumerator5"))

(fn `deathFX`
  (locals (fx :type "NiagaraComponent Object Reference"))
  (bind _returnvalue (`NiagaraFunctionLibrary.SpawnSystemAtLocation` "/Game/FX/NS_EnemyDead.NS_EnemyDead" (`self.K2_GetActorLocation`) (struct) (1.0 1.0 1.0) true false))
  (bind _output_get (set `local.fx` _returnvalue))
  (`NiagaraComponent.SetVariableFloat` _output_get "cylHeight" (* (`self.getWorldHalfHeight`) 2.0))
  (`NiagaraComponent.SetVariableFloat` (`local.fx`) "cylRadius" (`CapsuleComponent.GetScaledCapsuleRadius` (`self.Capsule`)))
  (`ActorComponent.Activate` (`local.fx`) true))

(fn `facePlayer`
  (params (rotateZ :type Boolean))
  (`self.K2_SetActorRotation` (`self.facingPlayerRotation` rotateZ)))

(fn `facingPlayerRotation`
  (params (rotateZ :type Boolean))
  (returns (ReturnValue :type "Rotator Structure"))
  (bind (_returnvalue_x _returnvalue_y _returnvalue_z) (`KismetMathLibrary.BreakVector` (`self.K2_GetActorLocation`)))
  (bind (_returnvalue_x_2 _returnvalue_y_2 _returnvalue_z_2) (`KismetMathLibrary.BreakVector` (`/Game/Blueprints/Enemies/BPC_EnemyAI.getPlayerLocation` (`self.BPC_EnemyAI`) false)))
  (return (`KismetMathLibrary.FindLookAtRotation` (`KismetMathLibrary.MakeVector` _returnvalue_x _returnvalue_y (`KismetMathLibrary.SelectFloat` _returnvalue_z 0.0 (`local.rotateZ`))) (`KismetMathLibrary.MakeVector` _returnvalue_x_2 _returnvalue_y_2 (`KismetMathLibrary.SelectFloat` _returnvalue_z_2 0.0 (`local.rotateZ`))))))

(fn `fireBeam`
  (params (fireFrom :type "Vector Structure") (target :type "Vector Structure") (maxDistance :type "Float (single-precision)" :default 3000.0) (printDebug :type Boolean))
  (`|SpawnActorFromClass` "/Game/Blueprints/Enemies/Actions/Attack/BP_EnemyBeam.BP_EnemyBeam_C" (`KismetMathLibrary.MakeTransform` fireFrom) "Undefined" "MultiplyWithRoot" self fireFrom (+ fireFrom (* (`KismetMathLibrary.Conv_RotatorToVector` (`KismetMathLibrary.FindLookAtRotation` fireFrom target)) (`local.maxDistance`))) printDebug null))

(fn `firstBeatOfAttack`
  (`self.newBeatOfAttack` (`self.getRandomValidAttackID`) 1))

(fn `getAttackByID`
  (params (ID :type Integer))
  (returns (Output :type "/Game/Blueprints/Enemies/Actions/Attack/SAttackInfo Structure (by ref)"))
  (return (`|GetArrayItem` (`self.attackInfo`) ID)))

(fn `getBeatOfAttack`
  (params (attack :type "/Game/Blueprints/Enemies/Actions/Attack/SAttackInfo Structure (by ref)") (beat :type Integer))
  (returns (Output :type "/Game/Blueprints/Enemies/Actions/Attack/SAttackBeatInfo Structure (by ref)"))
  (return (`|GetArrayItem` (`.attackBeats_3_A9E7663F4D5B2382F55D498B4FD5A02F` (break `/Game/Blueprints/Enemies/Actions/Attack/SAttackInfo` attack)) (- beat 1))))

(fn `getCurrentAttackLength`
  (returns (ReturnValue :type Integer))
  (return (`KismetArrayLibrary.Array_Length` (`.attackBeats_3_A9E7663F4D5B2382F55D498B4FD5A02F` (break `/Game/Blueprints/Enemies/Actions/Attack/SAttackInfo` (`|GetArrayItem` (`self.attackInfo`) (`self.currentAttackID`)))))))

(fn `getJumpToHeight`
  (params (targetHeight :type "Float (double-precision)" :default 300.0))
  (returns (jumpPoint :type "Vector Structure"))
  (locals (colliderTop :type "Vector Structure" :default (0.0 0.0 0.0)) (capsuleHeight :type "Float (double-precision)"))
  (bind _collidertop (`local.colliderTop`))
  (bind (_x _y _z) (`KismetMathLibrary.BreakVector3f` (`self.K2_GetActorLocation`)))
  (set `local.capsuleHeight` (* (`self.getWorldHalfHeight`) 2.0))
  (set `local.colliderTop` (`KismetMathLibrary.MakeVector` _x _y (+ _z (`local.capsuleHeight`))))
  (bind (_outhit _returnvalue) (`KismetSystemLibrary.LineTraceSingle` _collidertop (+ _collidertop (* (`self.GetActorUpVector`) (`local.targetHeight`))) "TraceTypeQuery1"))
  (bind (_bblockinghit _binitialoverlap _time _distance _location _impactpoint _normal _impactnormal _physmat _hitactor _hitcomponent _hitbonename _bonename _hititem _elementindex _faceindex _tracestart _traceend) (`GameplayStatics.BreakHitResult` _outhit))
  (`KismetSystemLibrary.PrintString` (`KismetSystemLibrary.GetDisplayName` _hitactor))
  (bind (_x_2 _y_2 _z_2) (`KismetMathLibrary.BreakVector3f` (select `bool` _returnvalue :`false` _traceend :`true` _location)))
  (return (`KismetMathLibrary.MakeVector` _x_2 _y_2 (- _z_2 (`local.capsuleHeight`)))))

(fn `getNumberOfAttacks`
  (returns (ReturnValue :type Integer))
  (return (`KismetArrayLibrary.Array_Length` (`self.attackInfo`))))

(fn `getRandomValidAttackID`
  (returns (Output :type Integer))
  (bind _returnvalue (`self.getNumberOfAttacks`))
  (if (> _returnvalue 0)
    (return (`KismetMathLibrary.RandomIntegerInRange` 0 (- _returnvalue 1)))
    (else
      (return -1))))

(fn `getWorldHalfHeight`
  (returns (ReturnValue :type "Float (double-precision)"))
  (bind _capsule (`self.Capsule`))
  (bind (_returnvalue_x _returnvalue_y _returnvalue_z) (`KismetMathLibrary.BreakVector` (`SceneComponent.K2_GetComponentScale` _capsule)))
  (return (* (`CapsuleComponent.CapsuleHalfHeight` _capsule) _returnvalue_z)))

(fn `isAttacking`
  (returns (ReturnValue :type Boolean))
  (return (!= (`self.currentBeatOfAttack`) -1)))

(fn `jumpToHeight`
  (params (targetHeight :type "Float (double-precision)" :default 300.0) (rotateFacePlayerZ :type Boolean))
  (`self.moveToPoint` (`self.getJumpToHeight` targetHeight) (`self.facingPlayerRotation` rotateFacePlayerZ) false))

(fn `moveSetDistanceFromPlayer`
  (params (dist :type "Float (double-precision)" :default 200.0) (rotateZ :type Boolean) (damagePlayerRadius :type "Float (double-precision)") (damageToDeal :type Integer) (instakill :type Boolean))
  (`self.moveToPoint` (+ (`self.lastRememberedPlayerLocation`) (* (`KismetMathLibrary.Conv_RotatorToVector` (`KismetMathLibrary.NegateRotator` (`self.facingPlayerRotation` false))) (`local.dist`))) (`self.facingPlayerRotation` (`local.rotateZ`)) true damagePlayerRadius damageToDeal instakill))

(fn `moveToBestPoint`
  (params (facePlayer :type Boolean :default true))
  (`self.moveToPoint` (`/Game/Blueprints/Enemies/BPC_EnemyAI.findBestValidMovePoint` (`self.BPC_EnemyAI`) (`self.movementDistance`)) (`self.solveBestRotation` (`local.facePlayer`))))

(fn `moveToPoint`
  (params (movePoint :type "Vector Structure") (newRotation :type "Rotator Structure") (absoluteForceGrounded :type Boolean :default true) (damagePlayerRadius :type "Float (double-precision)") (damageToDeal :type Integer) (instakill :type Boolean))
  (bind (_x _y) (`KismetMathLibrary.BreakVector3f` movePoint))
  (bind (_returnvalue_x _returnvalue_y _returnvalue_z) (`KismetMathLibrary.BreakVector` (`/Game/Blueprints/Enemies/BPC_EnemyAI.getPlayerLocation` (`self.BPC_EnemyAI`) false)))
  (bind _returnvalue (`KismetMathLibrary.SelectVector` (`KismetMathLibrary.MakeVector` _x _y _returnvalue_z) (`local.movePoint`) (`local.absoluteForceGrounded`)))
  (`self.updateLineRendererPositionPt1`)
  (if (`self.lerpMovement`)
    (`self.K2_SetActorRotation` (`local.newRotation`))
    (`self.LerpToSpot` _returnvalue damagePlayerRadius damageToDeal instakill)
    (else
      (`self.K2_SetActorLocationAndRotation` _returnvalue (`local.newRotation`))
      (`self.updateLineRendererPositionPt2`))))

(fn `newBeatOfAttack`
  (params (attackID :type Integer) (beatOfAttack :type Integer))
  (locals (attackBeat :type "/Game/Blueprints/Enemies/Actions/Attack/SAttackBeatInfo Structure"))
  (bind (_type _anim) (break `/Game/Blueprints/Enemies/Actions/Attack/SAttackBeatInfo` (`local.attackBeat`)))
  (set `local.attackBeat` (`self.getBeatOfAttack` (`self.getAttackByID` attackID) (`local.beatOfAttack`)))
  (`self.setAnim` _anim)
  (`self.attackBeatTypeEffects` _type))

(fn `setAnim`
  (params (anim :type "AnimSequence Object Reference"))
  (bind _enemyskeletalmesh (`self.EnemySkeletalMesh`))
  (`self.playAnimation` _enemyskeletalmesh anim)
  (`SceneComponent.SetRelativeScale3D` _enemyskeletalmesh (`KismetMathLibrary.Conv_DoubleToVector` 100.0)))

(fn `solveBestRotation`
  (params (facePlayer :type Boolean :default true) (rotateZ :type Boolean))
  (returns (ReturnValue :type "Rotator Structure"))
  (return (`KismetMathLibrary.SelectRotator` (`self.facingPlayerRotation` rotateZ) (`self.K2_GetActorRotation`) facePlayer)))

(fn `spawnAlign`
  (bind _returnvalue (`self.K2_GetActorLocation`))
  (`self.moveToPoint` (`/Game/Blueprints/Enemies/BPC_EnemyAI.validateMovePoint` (`self.BPC_EnemyAI`) _returnvalue (`self.movementDistance`) (`.ReturnValue` (`/Game/Blueprints/Enemies/BPC_EnemyAI.isPointInTargetDist` (`self.BPC_EnemyAI`) _returnvalue))) (`self.solveBestRotation` (`self.facePlayerOnSpawn`))))

(fn `spawnPreattackFX`
  (bind _enemyskeletalmesh (`self.EnemySkeletalMesh`))
  (bind _returnvalue (`|SpawnActorFromClass` "/Game/FX/BP_PreattackFX.BP_PreattackFX_C" (`KismetMathLibrary.MakeTransform` (+ (`SceneComponent.K2_GetComponentLocation` (`self.InteractionTransform`)) (* (`SceneComponent.GetRightVector` _enemyskeletalmesh) -150.0)) (`SceneComponent.K2_GetComponentRotation` _enemyskeletalmesh)) "Undefined" "MultiplyWithRoot" null null))
  (`self.K2_AttachToComponent` _returnvalue (`self.Capsule`) "None" "KeepWorld" "KeepWorld" "KeepWorld" true))

(fn `updateAttackBeat`
  (if (!= (`self.currentBeatOfAttack`) -1)
    (bind _result (`/Engine/EditorBlueprintResources/StandardMacros.IncrementInt` (`self.currentBeatOfAttack`))
      (:`  `
        (if (> _result (`self.getCurrentAttackLength`))
          (set `self.currentBeatOfAttack` -1)
          (`self.setAnim` (`self.idleAnim`))
          (else
            (`self.newBeatOfAttack` (`self.currentAttackID`) (`self.currentBeatOfAttack`))))))))

(fn `updateCollisionOffsets`
  (bind _returnvalue (`self.getWorldHalfHeight`))
  (bind _capsule (`self.Capsule`))
  (bind (_returnvalue_x _returnvalue_y) (`KismetMathLibrary.BreakVector` (* (`SceneComponent.K2_GetComponentScale` _capsule) (`SceneComponent.RelativeLocation` _capsule))))
  (`SceneComponent.K2_SetRelativeLocation` (`self.Capsule`) (`KismetMathLibrary.MakeVector` _returnvalue_x _returnvalue_y _returnvalue) false false)
  (`SceneComponent.K2_SetRelativeLocation` (`self.EnemySkeletalMesh`) (`KismetMathLibrary.MakeVector` 0.0 0.0 (* _returnvalue -1.0)) false false)
  (`SceneComponent.K2_SetRelativeLocation` (`self.InteractionTransform`) (`KismetMathLibrary.MakeVector` 0.0 0.0 _returnvalue) false false)
  (`SceneComponent.K2_SetRelativeLocation` (`self.DefeatHint`) (`KismetMathLibrary.MakeVector` 0.0 0.0 (+ _returnvalue (`self.defeatHintZOffset`))) false false))

(fn `updateDefeatHint`
  (bind _defeattype (`self.defeatType`))
  (`SceneComponent.SetVisibility` (`self.DefeatHint`) (`self.displayDefeatHint`) false)
  (if (`self.displayDefeatHint`)
    (`/Game/UI/BP_TitleBodyText.setText` (cast `/Game/UI/BP_TitleBodyText` (`ChildActorComponent.ChildActor` (`self.DefeatHint`)) :!pure true) (select `/Game/Blueprints/Enemies/_EnemyTypes/EEnemyDefeatType` _defeattype :`NewEnumerator0` "ROBOT" :`NewEnumerator1` "HUMAN" :`NewEnumerator2` "SQUID" :!type "Text") (select `/Game/Blueprints/Enemies/_EnemyTypes/EEnemyDefeatType` _defeattype :`NewEnumerator0` "Defeat with Liquid" :`NewEnumerator1` "Defeat with Electricity" :`NewEnumerator2` "Create your own electrocution" :!type "Text"))))

(fn `updateLastRememberedPlayerPosition`
  (params (useCameraPos :type Boolean))
  (set `self.lastRememberedPlayerLocation` (`/Game/Blueprints/Enemies/BPC_EnemyAI.getPlayerLocation` (`self.BPC_EnemyAI`) useCameraPos)))

(fn `updateLineRendererPositionPt1`
  (set `self.previousLocation` (`SceneComponent.K2_GetComponentLocation` (`self.InteractionTransform`))))

(fn `updateLineRendererPositionPt2`
  (bind _interactiontransform (`self.InteractionTransform`)
    (:`then`
      (`FXSystemComponent.SetVectorParameter` (`self.NS_EnemyMove`) "lastPos" (- (`self.previousLocation`) (`SceneComponent.K2_GetComponentLocation` _interactiontransform)))
      (`ActorComponent.Activate` (`self.NS_EnemyMove`) false))
    (:`else`)))

(fn `UserConstructionScript`
  (`parent.UserConstructionScript`)
  (`self.updateCollisionOffsets`)
  (`self.updateDefeatHint`)
  (`self.setMeshes` (`|MakeArray` (`self.EnemySkeletalMesh`) :!type "MeshComponent Object Reference"))
  (`self.setAnim` (`self.idleAnim`)))