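; Enemy AI component for beat-timed combat that registers its owning BP_EnemyBase with a shared hivemind after a beat-aligned delay.
; Each beat counts down move and attack cooldowns, refreshes player distance and advances the enemy's beat logic.
; It offers its highest-weighted valid action and executes moves or attacks on request.
; Moves retreat, approach or strafe by distance band, falling back to a random navigable point or standing still.
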(event `self.ReceiveBeginPlay`
  (set `self.parentEnemy` (cast `/Game/Blueprints/Enemies/BP_EnemyBase` (`self.GetOwner`) :!pure true))
  (`KismetSystemLibrary.K2_SetTimerDelegate` (delegate `Join Hivemind`) (`/Game/Blueprints/BPFL_BlueprintFunctionLibrary.getBeatStartDelay` true)))

(event `Join Hivemind`
  (bind _output_get (set `self.hivemind` (`/Game/Blueprints/BPFL_BlueprintFunctionLibrary.getAIHivemind`)))
  (`/Game/Blueprints/Enemies/BP_AIHivemind.addToHivemind` _output_get self))

(event `self.ReceiveEndPlay`
  (params (EndPlayReason :type "EEndPlayReason Enum" :default "Destroyed"))
  (`/Game/Blueprints/Enemies/BP_AIHivemind.removeFromHivemind` (`self.hivemind`) self))

(event `OnBeat`
  (`self.updateStatus`)
  (`/Game/Blueprints/Enemies/BP_EnemyBase.updateAttackBeat` (`self.parentEnemy`))
  (`/Game/Blueprints/Enemies/BP_EnemyBase.OnBeat` (`self.parentEnemy`)))

(event `OnMove`
  (set `self.beatsTillCanMove` (`/Game/Blueprints/Enemies/BP_EnemyBase.movementSpeedInBeats` (`self.parentEnemy`)))
  (set `self.canMoveNow` false))

(event `OnAttack`
  (set `self.beatsTillCanAttack` (+ (`/Game/Blueprints/Enemies/BP_EnemyBase.getCurrentAttackLength` (`self.parentEnemy`)) (`KismetMathLibrary.RandomIntegerInRange` (`self.minBeatsBtwnAttacks`) (`self.maxBeatsBtwnAttacks`))))
  (set `self.canAttackNow` false))

(fn `findBestValidMovePoint`
  (params (mvmtDist :type "Float (double-precision)" :default 300.0))
  (returns (movePoint :type "Vector Structure"))
  (locals (parentLocation :type "Vector Structure" :default (0.0 0.0 0.0)))
  (bind _output_get (set `local.parentLocation` (`Actor.K2_GetActorLocation` (`self.parentEnemy`))))
  (bind (_distfromplayer _returnvalue) (`self.isPointInTargetDist` _output_get))
  (return (`self.validateMovePoint` (+ (* (`self.getDirectionalMvmtVectorFromPlayer` _returnvalue) (`local.mvmtDist`)) (`local.parentLocation`)) (`local.mvmtDist`) _returnvalue)))

(fn `getDirectionalMvmtVectorFromPlayer`
  (params (targetDistState :type "/Game/Blueprints/Enemies/Actions/ETargetDist Enum" :default "NewEnumerator0") (forceZToPlayer :type Boolean))
  (returns (directionalVector :type "Vector Structure"))
  (bind _returnvalue (`KismetMathLibrary.GetForwardVector` (`KismetMathLibrary.FindLookAtRotation` (`self.getPlayerLocation` false) (`Actor.K2_GetActorLocation` (`self.parentEnemy`)))))
  (bind _returnvalue_2 (`SceneComponent.GetRightVector` (`/Game/VRTemplate/Blueprints/VRPawn.Camera` (`/Game/Blueprints/Enemies/BP_AIHivemind.player` (`self.hivemind`)))))
  (bind _returnvalue_3 (select `/Game/Blueprints/Enemies/Actions/ETargetDist` targetDistState :`NewEnumerator0` (`KismetMathLibrary.SelectVector` _returnvalue_2 (`KismetMathLibrary.NegateVector` _returnvalue_2) (`KismetMathLibrary.RandomBool`)) :`NewEnumerator1` _returnvalue :`NewEnumerator2` (`KismetMathLibrary.NegateVector` _returnvalue)))
  (bind (_x _y) (`KismetMathLibrary.BreakVector3f` _returnvalue_3))
  (`/Game/Blueprints/Enemies/BP_AIHivemind.player` (`self.hivemind`)
    (:`then`
      (return (`KismetMathLibrary.Normal` (`KismetMathLibrary.SelectVector` (`KismetMathLibrary.MakeVector` _x _y) _returnvalue_3 (`local.forceZToPlayer`)))))
    (:`else`
      (return (0.0 0.0 0.0)))))

(fn `getHeaviestValidAction`
  (returns (actionWeight :type "/Game/Blueprints/Enemies/Actions/SActionWeight Structure"))
  (locals (heaviestWeight :type "Float (double-precision)" :default 0.0) (heaviestAction :type "/Game/Blueprints/Enemies/Actions/EEnemyActionType Enum"))
  (if (not (`self.isEnemyAttacking`))
    (bind _keys (`BlueprintMapLibrary.Map_Keys` (`self.actionWeights`))) ; keys = actions
    (for _array_element _keys
      (bind _value (`BlueprintMapLibrary.Map_Find` (`self.actionWeights`) _array_element))
      (if (and (`self.isActionConditionMet` _array_element) (> _value (`local.heaviestWeight`)))
        (set `local.heaviestWeight` _value)
        (set `local.heaviestAction` _array_element)))
    (return (make `/Game/Blueprints/Enemies/Actions/SActionWeight` (`local.heaviestAction`) (`local.heaviestWeight`) self))
    (else
      (return (make `/Game/Blueprints/Enemies/Actions/SActionWeight` "NewEnumerator0" 1.0 self)))))

(fn `getPlayerLocation`
  (params (useCameraPos :type Boolean))
  (returns (ReturnValue :type "Vector Structure"))
  (bind _hivemind (`self.hivemind`)
    (:`then`
      _)
    (:`else`
      (`self.Join Hivemind`)
      (`self.hivemind`
        (:`then`
          _)
        (:`else`
          (return (`Actor.K2_GetActorLocation` (`GameplayStatics.GetPlayerPawn` 0)))))))
  (return (`/Game/Blueprints/Enemies/BP_AIHivemind.getPlayerLocation` _hivemind (`local.useCameraPos`))))

(fn `isActionConditionMet`
  (params (action :type "/Game/Blueprints/Enemies/Actions/EEnemyActionType Enum" :default "NewEnumerator0"))
  (returns (ReturnValue :type Boolean))
  (bind _canmovenow (`self.canMoveNow`))
  (return (and (not (`/Game/Blueprints/Interactive/BPC_Interactive.hasProperty` (`/Game/Blueprints/Interactive/BP_InteractiveBase.BPC_Interactive` (`self.parentEnemy`)) "NewEnumerator10")) (select `/Game/Blueprints/Enemies/Actions/EEnemyActionType` (`local.action`) :`NewEnumerator0` true :`NewEnumerator1` (and (`self.inTargetDist`) _canmovenow) :`NewEnumerator3` (and (not (`self.inTargetDist`)) _canmovenow) :`NewEnumerator2` (and (`self.canAttackNow`) (not (`self.isEnemyAttacking`))) :`NewEnumerator4` true))))

(fn `isEnemyAttacking`
  (returns (ReturnValue :type Boolean))
  (return (`/Game/Blueprints/Enemies/BP_EnemyBase.isAttacking` (`self.parentEnemy`))))

(fn `isEnemyInTargetDist`
  (returns (distFromPlayer :type "Float (double-precision)") (inTargetDist :type Boolean))
  (bind (_distfromplayer _returnvalue) (`self.isPointInTargetDist` (`Actor.K2_GetActorLocation` (`self.parentEnemy`))))
  (return _distfromplayer (`|EnumEquality` _returnvalue "NewEnumerator0")))

(fn `isPointInTargetDist`
  (params (location :type "Vector Structure"))
  (returns (distFromPlayer :type "Float (double-precision)") (ReturnValue :type "/Game/Blueprints/Enemies/Actions/ETargetDist Enum"))
  (locals (dist :type "Float (double-precision)" :default 0.0))
  (set `local.dist` (`KismetMathLibrary.Vector_Distance` location (`self.getPlayerLocation` false)))
  (if (< (`local.dist`) (`self.minTargetDistFromPlayer`))
    (return (`local.dist`) "NewEnumerator1")
    (elif (> (`local.dist`) (`self.maxTargetDistFromPlayer`))
      (return (`local.dist`) "NewEnumerator2")
      (else
        (return (`local.dist`) "NewEnumerator0")))))

(fn `performAction`
  (params (action :type "/Game/Blueprints/Enemies/Actions/EEnemyActionType Enum" :default "NewEnumerator0"))
  (`self.parentEnemy`
    (:`then`
      (if (`self.printDebugInformation`)
        (`KismetSystemLibrary.PrintString` (`KismetStringLibrary.Concat_StrStr` (`KismetSystemLibrary.GetDisplayName` (`self.parentEnemy`)) " performs " (`|GetEnumeratorNameAsString` (`local.action`))) true true (struct :`G` 1.0 :`B` 0.635175 :`A` 1.0) 4.0))
      (switch `/Game/Blueprints/Enemies/Actions/EEnemyActionType` action
        (:`NewEnumerator1`
          (`/Game/Blueprints/Enemies/BP_EnemyBase.moveToBestPoint` (`self.parentEnemy`) true :!label _label)
          (`/Game/Blueprints/Enemies/BP_EnemyBase.MoveStart` (`self.parentEnemy`))
          (`self.OnMove`))
        (:`NewEnumerator3`
          (goto _label))
        (:`NewEnumerator2`
          (set `/Game/Blueprints/Enemies/BP_EnemyBase.currentBeatOfAttack` 1 (`self.parentEnemy`))
          (`/Game/Blueprints/Enemies/BP_EnemyBase.firstBeatOfAttack` (`self.parentEnemy`))
          (`/Game/Blueprints/Enemies/BP_EnemyBase.AttackStart` (`self.parentEnemy`))
          (`self.OnAttack`))))
    (:`else`)))

(fn `updateBeatsTillCanAttack`
  (if (> (`self.beatsTillCanAttack`) 0)
    (`/Engine/EditorBlueprintResources/StandardMacros.DecrementInt` (`self.beatsTillCanAttack`)
      (:`  `
        (set `self.canAttackNow` (== (`self.beatsTillCanAttack`) 0))))))

(fn `updateBeatsTillCanMove`
  (if (> (`self.beatsTillCanMove`) 0)
    (`/Engine/EditorBlueprintResources/StandardMacros.DecrementInt` (`self.beatsTillCanMove`)
      (:`  `
        (set `self.canMoveNow` (== (`self.beatsTillCanMove`) 0))))))

(fn `updateStatus`
  (bind (_distfromplayer _intargetdist) (`self.isEnemyInTargetDist`))
  (`|ExecutionSequence`
    (:`then_0`
      (`self.updateBeatsTillCanMove`)
      (set `self.distFromPlayer` _distfromplayer)
      (set `self.inTargetDist` _intargetdist))
    (:`then_1`
      (`self.updateBeatsTillCanAttack`))))

(fn `validateMovePoint`
  (params (desiredPoint :type "Vector Structure") (mvmtDist :type "Float (double-precision)" :default 300.0) (targetDist :type "/Game/Blueprints/Enemies/Actions/ETargetDist Enum" :default "NewEnumerator0"))
  (returns (movePoint :type "Vector Structure"))
  (locals (parentLocation :type "Vector Structure" :default (0.0 0.0 0.0)) (randomPoint :type "Vector Structure" :default (0.0 0.0 0.0)))
  (set `local.parentLocation` (`Actor.K2_GetActorLocation` (`self.parentEnemy`)))
  ;[0.2995 1 0.2938] Move to desired position. Best case.
  (if (`|EnumEquality` (`.ReturnValue` (`NavigationSystemV1.GetPathLength` (`local.parentLocation`) (`local.desiredPoint`) null null)) "Success")
    (if (`self.printDebugInformation`)
      (`KismetSystemLibrary.PrintString` (`KismetStringLibrary.Concat_StrStr` (`KismetSystemLibrary.GetDisplayName` (`self.parentEnemy`)) " succesfully moves, was target dist " (`|GetEnumeratorNameAsString` (`local.targetDist`))) true true (struct :`G` 0.3 :`A` 1.0) 5.0))
    (return (`local.desiredPoint`))
    (else
      ;[0.9313 1 0.2514] Use random navigable point. Mid case.
      (bind (_randomlocation _returnvalue) (`NavigationSystemV1.K2_GetRandomLocationInNavigableRadius` (`local.parentLocation`) (`local.mvmtDist`) null null))
      (set `local.randomPoint` _randomlocation)
      (if _returnvalue
        (if (`|EnumEquality` (`.ReturnValue` (`NavigationSystemV1.GetPathLength` (`local.parentLocation`) (`local.randomPoint`) null null)) "Success")
          (if (`self.printDebugInformation`)
            (`KismetSystemLibrary.PrintString` (`KismetStringLibrary.Concat_StrStr` (`KismetSystemLibrary.GetDisplayName` (`self.parentEnemy`)) " fails to move on target dist " (`|GetEnumeratorNameAsString` (`local.targetDist`)) ". Uses random instead") true true (struct :`R` 0.3 :`G` 0.3 :`A` 1.0) 5.0))
          (return (`local.randomPoint`))
          (else
            _)))
      ;[1 0.2198 0.2583] Do not move. Worst case.
      (if (`self.printDebugInformation`)
        (`KismetSystemLibrary.PrintString` (`KismetStringLibrary.Concat_StrStr` (`KismetSystemLibrary.GetDisplayName` (`self.parentEnemy`)) " fully fails target dist " (`|GetEnumeratorNameAsString` (`local.targetDist`)) " and random. No move.") true true (struct :`R` 0.3 :`A` 1.0) 5.0))
      (return (`local.parentLocation`)))))