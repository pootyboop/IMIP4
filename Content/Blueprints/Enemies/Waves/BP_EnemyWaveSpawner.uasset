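; Trigger-box spawner that runs waves of enemies, starting when the VR pawn first enters and registering itself as the active spawner.
; Each wave spawns through the AI hivemind at random points around the box's center, then refreshes music tracks.
; Kills update per-type counts; when the enemy count hits zero, a countdown on rhythm beats launches the next wave.
; The spawner deactivates after the last wave.
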(event `self.ReceiveBeginPlay`
  (set `self.hivemind` (`/Game/Blueprints/BPFL_BlueprintFunctionLibrary.getAIHivemind`))
  (`KismetSystemLibrary.K2_SetTimerDelegate` (delegate `SetupBeats`) (`/Game/Blueprints/BPFL_BlueprintFunctionLibrary.getBeatStartDelay` true)))

(event `SetupBeats`
  (`/Game/Blueprints/BPFL_BlueprintFunctionLibrary.bindEventToRhythm` "NewEnumerator1" (delegate `OnBeat`)))

(event `OnBeat`
  (if (and (!= (`self.beatsTillNextWave`) 0) (`self.active`))
    (bind _result (`/Engine/EditorBlueprintResources/StandardMacros.DecrementInt` (`self.beatsTillNextWave`))
      (:`  `
        (if (== _result 0)
          (`self.NextWave`))))))

(event `self.Box.OnComponentBeginOverlap`
  (params (OverlappedComponent :type "PrimitiveComponent Object Reference") (OtherActor :type "Actor Object Reference") (OtherComp :type "PrimitiveComponent Object Reference") (OtherBodyIndex :type Integer) (bFromSweep :type Boolean) (SweepResult :type "HitResult Structure (by ref)"))
  (if (== (`GameplayStatics.GetObjectClass` OtherActor) "/Game/VRTemplate/Blueprints/VRPawn.VRPawn_C")
    (if (== (`self.currWave`) 0)
      (set `self.active` true)
      (`/Game/Blueprints/GI_GameInstance.setActiveSpawner` (`/Game/Blueprints/BPFL_BlueprintFunctionLibrary.getGI`) self)
      (`self.NextWave`))))

(event `NextWave`
  (bind _result (`/Engine/EditorBlueprintResources/StandardMacros.IncrementInt` (`self.currWave`))
    (:`  `
      (if (<= _result (`KismetArrayLibrary.Array_Length` (`self.waves`)))
        (`self.spawnEnemies` (`.enemies_3_FAEBD7A74BC9EFD0692E199577B3E112` (break `/Game/Blueprints/Enemies/Waves/SWave` (`|GetArrayItem` (`self.waves`) (- (`self.currWave`) 1)))))
        (else
          (`self.AllWavesCleared`))))))

(event `WaveCleared`
  (set `self.beatsTillNextWave` (`self.beatsBetweenClearAndNewWave`)))

(event `AllWavesCleared`
  (set `self.active` false)
  (`/Game/Blueprints/GI_GameInstance.setActiveSpawner` (`/Game/Blueprints/BPFL_BlueprintFunctionLibrary.getGI`) null))

(fn `enemyKilled`
  (params (type :type "/Game/Blueprints/Enemies/_EnemyTypes/EEnemyType Enum" :default "NewEnumerator0"))
  (`/Engine/EditorBlueprintResources/StandardMacros.DecrementInt` (`self.enemyCount`)
    (:`  `
      (`|ExecutionSequence`
        (:`then_0`
          (`self.modifyEnemyTypeCt` (`local.type`) -1))
        (:`then_1`
          (if (== (`self.enemyCount`) 0)
            (`self.WaveCleared`)))))))

(fn `getEnemyTypeCt`
  (params (enemyType :type "/Game/Blueprints/Enemies/_EnemyTypes/EEnemyType Enum" :default "NewEnumerator0"))
  (returns (Value :type Integer))
  (bind (_value _returnvalue) (`BlueprintMapLibrary.Map_Find` (`self.enemyTypesRegister`) enemyType))
  (if _returnvalue
    (return _value)
    (else
      (return 0))))

(fn `modifyEnemyTypeCt`
  (params (enemyType :type "/Game/Blueprints/Enemies/_EnemyTypes/EEnemyType Enum" :default "NewEnumerator0") (count :type Integer))
  (returns (newCount :type Integer) (success :type Boolean))
  (locals (newCt :type Integer))
  (bind _output_get (set `local.newCt` (+ (`BlueprintMapLibrary.Map_Find` (`self.enemyTypesRegister`) enemyType) (`local.count`))))
  (`BlueprintMapLibrary.Map_Add` (`self.enemyTypesRegister`) (`local.enemyType`) _output_get)
  (return (`local.newCt`) true))

(fn `randomSpawnPointInBox`
  (returns (ReturnValue :type "Vector Structure"))
  (bind _box (`self.Box`))
  (bind (_returnvalue_x _returnvalue_y) (`KismetMathLibrary.BreakVector` (`SceneComponent.K2_GetComponentScale` _box)))
  (bind (_boxextent_x _boxextent_y) (`KismetMathLibrary.BreakVector` (`BoxComponent.BoxExtent` _box)))
  (return (`KismetMathLibrary.RandomPointInBoundingBox` (`self.K2_GetActorLocation`) (`KismetMathLibrary.MakeVector` (* _boxextent_x 0.5 _returnvalue_x) (* _boxextent_y 0.5 _returnvalue_y)))))

(fn `spawnEnemies`
  (params (enemies :type "Array of /Game/Blueprints/Enemies/Waves/SWaveEnemy Structure"))
  (`self.hivemind`
    (:`then`
      _)
    (:`else`
      (set `self.hivemind` (`/Game/Blueprints/BPFL_BlueprintFunctionLibrary.getAIHivemind`))))
  (for _array_element (`local.enemies`)
    (bind (_enemytype _number) (break `/Game/Blueprints/Enemies/Waves/SWaveEnemy` _array_element))
    (for _ (range _number)
      (`/Game/Blueprints/Enemies/BP_AIHivemind.spawnEnemy` (`self.hivemind`) _enemytype (`KismetMathLibrary.Conv_VectorToTransform` (`self.randomSpawnPointInBox`)) true self)
      (`self.modifyEnemyTypeCt` _enemytype 1)))
  (set `self.enemyCount` (`KismetArrayLibrary.Array_Length` (`local.enemies`)))
  (`/Game/Blueprints/BPFL_BlueprintFunctionLibrary.refreshMusicTracks`))

(fn `UserConstructionScript`
  (`SceneComponent.SetHiddenInGame` (`self.Box`) (`self.hitboxHidden`) false))