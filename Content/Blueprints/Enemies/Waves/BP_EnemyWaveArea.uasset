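; BP_EnemyWaveArea is a box trigger area that spawns the first enemy wave when the VRPawn first enters it.
; NextWave advances the wave counter and spawns that entry of the Waves array; later waves need further NextWave calls from outside this graph.
; Each enemy spawns through the AI Hivemind, facing the player, at a random point within the inner half of the box's scaled X/Y extents.
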(event `self.ReceiveBeginPlay`
  (set `self.hivemind` (`/Game/Blueprints/BPFL_BlueprintFunctionLibrary.getAIHivemind`)))

(event `self.Box.OnComponentBeginOverlap`
  (params (OverlappedComponent :type "PrimitiveComponent Object Reference") (OtherActor :type "Actor Object Reference") (OtherComp :type "PrimitiveComponent Object Reference") (OtherBodyIndex :type Integer) (bFromSweep :type Boolean) (SweepResult :type "HitResult Structure (by ref)"))
  (if (== (`GameplayStatics.GetObjectClass` OtherActor) "/Game/VRTemplate/Blueprints/VRPawn.VRPawn_C")
    (if (== (`self.currWave`) 0)
      (`self.NextWave`))))

(event `self.Box.OnComponentEndOverlap`
  (params (OverlappedComponent :type "PrimitiveComponent Object Reference") (OtherActor :type "Actor Object Reference") (OtherComp :type "PrimitiveComponent Object Reference") (OtherBodyIndex :type Integer)))

(event `NextWave`
  (bind _result (`/Engine/EditorBlueprintResources/StandardMacros.IncrementInt` (`self.currWave`))
    (:`  `
      (`self.spawnEnemies` (`.enemies_3_FAEBD7A74BC9EFD0692E199577B3E112` (break `/Game/Blueprints/Enemies/Waves/SWave` (`|GetArrayItem` (`self.waves`) (- _result 1))))))))

(fn `randomSpawnPointInBox`
  (returns (ReturnValue :type "Vector Structure"))
  (bind _box (`self.Box`))
  (bind (_returnvalue_x _returnvalue_y) (`KismetMathLibrary.BreakVector` (`SceneComponent.K2_GetComponentScale` _box)))
  (bind (_boxextent_x _boxextent_y) (`KismetMathLibrary.BreakVector` (`BoxComponent.BoxExtent` _box)))
  (return (`KismetMathLibrary.RandomPointInBoundingBox` (`self.K2_GetActorLocation`) (`KismetMathLibrary.MakeVector` (* _boxextent_x 0.5 _returnvalue_x) (* _boxextent_y 0.5 _returnvalue_y)))))

(fn `spawnEnemies`
  (params (enemies :type "Array of /Game/Blueprints/Enemies/Waves/SWaveEnemy Structure"))
  (`self.hivemind`
    (:`then`
      _)
    (:`else`
      (set `self.hivemind` (`/Game/Blueprints/BPFL_BlueprintFunctionLibrary.getAIHivemind`))))
  (for _array_element (`local.enemies`)
    (bind (_enemytype _number) (break `/Game/Blueprints/Enemies/Waves/SWaveEnemy` _array_element))
    (for _ (range _number)
      (`/Game/Blueprints/Enemies/BP_AIHivemind.spawnEnemy` (`self.hivemind`) _enemytype (`KismetMathLibrary.Conv_VectorToTransform` (`self.randomSpawnPointInBox`)) true))))

(fn `UserConstructionScript`
  (`SceneComponent.SetHiddenInGame` (`self.Box`) (`self.hitboxHidden`) false))