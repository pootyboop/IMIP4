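; Central enemy AI coordinator that registers with the game instance and drives all enrolled enemies on the music rhythm.
; Each beat it notifies enemies, gathers each one's heaviest valid action and sorts them by weight.
; It executes only the top actions within per-type concurrency caps, counting attacks already underway against one type's cap.
; It also spawns Squid, Bishop or Butcher enemies and provides the VR player's location.
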(event `self.ReceiveBeginPlay`
  (`self.updateGIRef`)
  (`self.setupPlayer`)
  (`KismetSystemLibrary.K2_SetTimerDelegate` (delegate `BindBeatEvents`) (`/Game/Blueprints/BPFL_BlueprintFunctionLibrary.getBeatStartDelay` true)))

(event `BindBeatEvents`
  (`/Game/Blueprints/BPFL_BlueprintFunctionLibrary.bindEventToRhythm` "NewEnumerator1" (delegate `OnBeat`)))

(event `OnBeat`
  (`self.callEnemyAIBeats`)
  (`self.performEnemyActions`))

(fn `addToHivemind`
  (params (enemy :type "/Game/Blueprints/Enemies/BPC_EnemyAI Object Reference"))
  (`KismetArrayLibrary.Array_AddUnique` (`self.enemyAIs`) enemy))

(fn `callEnemyAIBeats`
  (for _array_element (`self.enemyAIs`)
    (`/Game/Blueprints/Enemies/BPC_EnemyAI.OnBeat` _array_element)))

(fn `classFromEnemyType`
  (params (enemyType :type "/Game/Blueprints/Enemies/_EnemyTypes/EEnemyType Enum" :default "NewEnumerator0"))
  (returns (class :type "/Game/Blueprints/Enemies/BP_EnemyBase Class Reference"))
  (return (select `/Game/Blueprints/Enemies/_EnemyTypes/EEnemyType` enemyType :`NewEnumerator0` "/Game/Blueprints/Enemies/_EnemyTypes/BP_Squid.BP_Squid_C" :`NewEnumerator1` "/Game/Blueprints/Enemies/_EnemyTypes/BP_Bishop.BP_Bishop_C" :`NewEnumerator2` "/Game/Blueprints/Enemies/_EnemyTypes/BP_Butcher.BP_Butcher_C" :!type "/Game/Blueprints/Enemies/BP_EnemyBase Class Reference")))

(fn `countCurrentConcurrentAttacks`
  (returns (attackingPerformers :type Integer))
  (locals (count :type Integer))
  (set `local.count` 0)
  (for _array_element (`self.enemyAIs`)
    (if (`/Game/Blueprints/Enemies/BPC_EnemyAI.isEnemyAttacking` _array_element)
      (`/Engine/EditorBlueprintResources/StandardMacros.IncrementInt` (`local.count`))))
  (return (`local.count`)))

(fn `getEnemyActions`
  (returns (actionWeights :type "Array of /Game/Blueprints/Enemies/Actions/SActionWeight Structure"))
  (locals (sactionWeights :type "Array of /Game/Blueprints/Enemies/Actions/SActionWeight Structure"))
  (for _array_element (`self.enemyAIs`)
    (bind _actionweight (`/Game/Blueprints/Enemies/BPC_EnemyAI.getHeaviestValidAction` _array_element))
    (if (`|EnumInequality` (`.action_3_E70C15384ABF0E1A30E66AAC2B89FDA8` (break `/Game/Blueprints/Enemies/Actions/SActionWeight` _actionweight)) "NewEnumerator0")
      (`KismetArrayLibrary.Array_Add` (`local.sactionWeights`) _actionweight)))
  (return (`local.sactionWeights`)))

(fn `getHeaviestActionsOfType`
  (params (preSortedActions :type "Array of /Game/Blueprints/Enemies/Actions/SActionWeight Structure") (actionType :type "/Game/Blueprints/Enemies/Actions/EEnemyActionType Enum" :default "NewEnumerator0") (maxNumToFind :type Integer))
  (returns (heaviestActions :type "Array of /Game/Blueprints/Enemies/Actions/SActionWeight Structure"))
  (locals (heavyActions :type "Array of /Game/Blueprints/Enemies/Actions/SActionWeight Structure") (numFound :type Integer))
  (`|ExecutionSequence`
    (:`then_0`
      (if (`|EnumEquality` (`local.actionType`) "NewEnumerator2")
        (set `local.numFound` (+ (`local.numFound`) (`self.countCurrentConcurrentAttacks`)))
        (if (>= (`local.numFound`) (`local.maxNumToFind`)) :!label _label
          (return (`local.heavyActions`)))))
    (:`then_1`
      (for _array_element (`local.preSortedActions`)
        (if (`|EnumEquality` (`.action_3_E70C15384ABF0E1A30E66AAC2B89FDA8` (break `/Game/Blueprints/Enemies/Actions/SActionWeight` _array_element)) (`local.actionType`))
          (`KismetArrayLibrary.Array_Add` (`local.heavyActions`) _array_element)
          (`/Engine/EditorBlueprintResources/StandardMacros.IncrementInt` (`local.numFound`)
            (:`  `
              (goto _label)))))
      (return (`local.heavyActions`)))))

(fn `getPlayerLocation`
  (params (useCameraPos :type Boolean))
  (returns (ReturnValue :type "Vector Structure"))
  (bind _player (`self.player`))
  (`self.player`
    (:`then`
      (return (`KismetMathLibrary.SelectVector` (`SceneComponent.K2_GetComponentLocation` (`/Game/VRTemplate/Blueprints/VRPawn.Camera` _player)) (`self.K2_GetActorLocation` _player) (`local.useCameraPos`))))
    (:`else`
      (bind _foundplayer (`self.setupPlayer`))
      (if _foundplayer
        (return (`KismetMathLibrary.SelectVector` (`SceneComponent.K2_GetComponentLocation` (`/Game/VRTemplate/Blueprints/VRPawn.Camera` _player)) (`self.K2_GetActorLocation` _player) (`local.useCameraPos`)))))))

(fn `performEnemyActions`
  (locals (actions :type "Array of /Game/Blueprints/Enemies/Actions/EEnemyActionType Enum") (actionWeights :type "Array of /Game/Blueprints/Enemies/Actions/SActionWeight Structure") (sortedActionWeights :type "Array of /Game/Blueprints/Enemies/Actions/SActionWeight Structure"))
  (`|ExecutionSequence`
    (:`then_0`
      ;[1 1 1] Get unsorted actions
      (bind _actionweights (`self.getEnemyActions`))
      (set `local.actionWeights` _actionweights))
    (:`then_1`
      ;[1 1 1] Sort each type of action by weight
      (bind _sortedactionweights (`self.sortActionsByWeight` (`local.actionWeights`)))
      (set `local.sortedActionWeights` _sortedactionweights))
    (:`then_2`
      ;[1 1 1] Perform final actions
      (bind _keys (`BlueprintMapLibrary.Map_Keys` (`self.maxConcurrentActionsByType`)))
      (for _array_element _keys
        (bind _heaviestactions (`self.getHeaviestActionsOfType` (`local.sortedActionWeights`) _array_element (`BlueprintMapLibrary.Map_Find` (`self.maxConcurrentActionsByType`) _array_element)))
        (for _array_element_2 _heaviestactions
          (bind (_action _weight _performer) (break `/Game/Blueprints/Enemies/Actions/SActionWeight` _array_element_2))
          (`/Game/Blueprints/Enemies/BPC_EnemyAI.performAction` _performer _action))))))

(fn `removeFromHivemind`
  (params (enemy :type "/Game/Blueprints/Enemies/BPC_EnemyAI Object Reference"))
  (`KismetArrayLibrary.Array_RemoveItem` (`self.enemyAIs`) enemy))

(fn `setupPlayer`
  (returns (foundPlayer :type Boolean))
  (`self.player`
    (:`then`
      (return true))
    (:`else`
      (bind _returnvalue (`GameplayStatics.GetActorOfClass` "/Game/VRTemplate/Blueprints/VRPawn.VRPawn_C"))
      (bind _output_get (set `self.player` _returnvalue))
      (return (`KismetSystemLibrary.IsValid` _output_get)))))

(fn `sortActionsByWeight`
  (params (inActions :type "Array of /Game/Blueprints/Enemies/Actions/SActionWeight Structure"))
  (returns (sortedActionWeights :type "Array of /Game/Blueprints/Enemies/Actions/SActionWeight Structure"))
  (locals (sortedActions :type "Array of /Game/Blueprints/Enemies/Actions/SActionWeight Structure") (weightArray :type "Array of Float (double-precision)") (actionArray :type "Array of /Game/Blueprints/Enemies/Actions/EEnemyActionType Enum") (performerArray :type "Array of /Game/Blueprints/Enemies/BPC_EnemyAI Object Reference"))
  (bind (_indexofmaxvalue _maxvalue) (`KismetMathLibrary.MaxOfFloatArray` (`local.weightArray`)))
  (`|ExecutionSequence`
    (:`then_0`
      (for _array_element inActions
        (bind (_action _weight _performer) (break `/Game/Blueprints/Enemies/Actions/SActionWeight` _array_element))
        (`KismetArrayLibrary.Array_Add` (`local.actionArray`) _action)
        (`KismetArrayLibrary.Array_Add` (`local.weightArray`) _weight)
        (`KismetArrayLibrary.Array_Add` (`local.performerArray`) _performer)))
    (:`then_1`
      (while (> (`KismetArrayLibrary.Array_Length` (`local.weightArray`)) 0)
        (`KismetArrayLibrary.Array_Add` (`local.sortedActions`) (make `/Game/Blueprints/Enemies/Actions/SActionWeight` (`|GetArrayItem` (`local.actionArray`) _indexofmaxvalue) _maxvalue (`|GetArrayItem` (`local.performerArray`) _indexofmaxvalue)))
        (`KismetArrayLibrary.Array_Remove` (`local.actionArray`) _indexofmaxvalue)
        (`KismetArrayLibrary.Array_Remove` (`local.weightArray`) _indexofmaxvalue)
        (`KismetArrayLibrary.Array_Remove` (`local.performerArray`) _indexofmaxvalue))
      (return (`local.sortedActions`)))))

(fn `spawnEnemy`
  (params (enemyType :type "/Game/Blueprints/Enemies/_EnemyTypes/EEnemyType Enum" :default "NewEnumerator0") (spawnTransform :type "Transform Structure") (spawnFacingPlayer :type Boolean))
  (returns (newEnemy :type "Actor Object Reference"))
  (bind _returnvalue (`|SpawnActorFromClass` (`self.classFromEnemyType` enemyType) (`local.spawnTransform`) "Undefined" "MultiplyWithRoot" null (`local.spawnFacingPlayer`) null))
  (return _returnvalue))

(fn `updateGIRef`
  (set `/Game/Blueprints/GI_GameInstance.aiHivemind` self (`/Game/Blueprints/BPFL_BlueprintFunctionLibrary.getGI`)))

(fn `UserConstructionScript`)