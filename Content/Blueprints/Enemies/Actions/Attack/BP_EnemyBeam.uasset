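; Short-lived enemy beam attack actor that fires a single instant hit when spawned and lasts until the next bound rhythm beat.
; FireBeam line traces from Source to Target, ignoring its owner, and stretches a colored electric Niagara beam to the impact point or trace end.
; A valid hit actor receives interact and damage messages.
; The rhythm callback then destroys the particles and the actor.
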(event `self.ReceiveBeginPlay`
  (`self.fireBeam`)
  (`/Game/Blueprints/BPFL_BlueprintFunctionLibrary.bindEventToRhythm` "NewEnumerator1" (delegate `OnBeat`)))

(event `OnBeat`
  (`ActorComponent.K2_DestroyComponent` (`self.particles`))
  (`self.K2_DestroyActor`))

(fn `fireBeam`
  (bind (_outhit _returnvalue) (`KismetSystemLibrary.LineTraceSingleByProfile` (`self.source`) (`self.target`) "None" false (`|MakeArray` (`self.GetOwner`))))
  (bind _returnvalue_2 (`NiagaraFunctionLibrary.SpawnSystemAtLocation` "/Game/FX/NS_EnemyBeam.NS_EnemyBeam" (`self.source`)))
  (bind _output_get (set `self.particles` _returnvalue_2))
  (bind (_bblockinghit _binitialoverlap _time _distance _location _impactpoint _normal _impactnormal _physmat _hitactor _hitcomponent _hitbonename _bonename _hititem _elementindex _faceindex _tracestart _traceend) (`GameplayStatics.BreakHitResult` _outhit))
  (`FXSystemComponent.SetVectorParameter` _output_get "BeamEnd" (- (`KismetMathLibrary.SelectVector` _location _traceend _returnvalue) (`self.source`)))
  (`/Game/Blueprints/BPFL_BlueprintFunctionLibrary.setElectricityColor` (`self.particles`))
  (bind _output_get_2 (set `self.hitActor` _hitactor))
  (`/Engine/EditorBlueprintResources/StandardMacros.IsValid` _output_get_2
    (:`Is Valid`
      (message `/Game/Blueprints/Interactive/BPI_Interactive.interactStart` (`self.hitActor`) null "NewEnumerator1")
      (bind _hitactor_2 (`self.hitActor`)
        (:`then`
          (message `/Game/Blueprints/Interactive/Destroyable/BPI_Destroyable.Damage` _hitactor_2 1 false "NewEnumerator5"))
        (:`else`
          _))
      (if (`self.printDebug`)
        (`KismetSystemLibrary.PrintString` (`KismetStringLibrary.Concat_StrStr` (`KismetSystemLibrary.GetDisplayName` (`self.GetOwner`)) " hit " (`KismetSystemLibrary.GetDisplayName` (`self.hitActor`))) true true (struct :`R` 0.5 :`G` 0.033333 :`B` 0.033333 :`A` 1.0))))))

(fn `UserConstructionScript`)