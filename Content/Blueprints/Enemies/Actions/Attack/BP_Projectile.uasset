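; Enemy attack projectile that, when thrown, detaches and flies to the first line-trace hit or the end of its range.
; A timeline lerps it there with a swept move and updates a Niagara trail.
; On arrival it damages the traced actor only if that actor has stayed within a dodge distance of its position at throw time.
; Rhythm binding, optionally delayed to beat start, destroys it on the first beat after arrival.
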(event `self.ReceiveBeginPlay`
  (if (`self.needsBeatBindEventDelay`)
    (`KismetSystemLibrary.K2_SetTimerDelegate` (delegate `SetupBeats`) (`/Game/Blueprints/BPFL_BlueprintFunctionLibrary.getBeatStartDelay` true))
    (else
      (`/Game/Blueprints/BPFL_BlueprintFunctionLibrary.bindEventToRhythm` "NewEnumerator1" (delegate `OnBeat`) :!label _label))))

(event `SetupBeats`
  (goto _label))

(event `OnBeat`
  (if (`self.thrown`)
    (`self.K2_DestroyActor`)))

(event `LerpToNewLoc`
  (bind (_direction _alpha) (`Timeline|Timeline` :!via `PlayFromStart`)
    (:`Update`
      (`self.K2_SetActorLocation` (`KismetMathLibrary.VLerp` (`self.prevLoc`) (`self.newLoc`) _alpha) true)
      (`self.updateTrail`))
    (:`Finished`
      (set `self.thrown` true)
      (`self.tryDamageHitActor`))))

(fn `throw`
  (params (direction :type "Vector Structure") (dist :type "Float (double-precision)" :default 1000.0) (destroy :type "/Game/Blueprints/Interactive/Destroyable/EDestroyableType Enum" :default "NewEnumerator5"))
  (locals (endLoc :type "Vector Structure" :default (0.0 0.0 0.0)))
  (`self.K2_DetachFromActor` "KeepWorld" "KeepWorld" "KeepWorld")
  (`self.K2_SetActorRotation` (`KismetMathLibrary.MakeRotFromX` (`local.direction`)))
  (bind _output_get (set `self.prevLoc` (`self.K2_GetActorLocation`)))
  (bind (_outhit _returnvalue) (`KismetSystemLibrary.LineTraceSingleByProfile` _output_get (+ _output_get (* (`local.direction`) (`local.dist`))) "None" false (`|MakeArray` (`self.GetOwner`))))
  (bind (_bblockinghit _binitialoverlap _time _distance _location _impactpoint _normal _impactnormal _physmat _hitactor _hitcomponent _hitbonename _bonename _hititem _elementindex _faceindex _tracestart _traceend) (`GameplayStatics.BreakHitResult` _outhit))
  (set `self.newLoc` (`KismetMathLibrary.SelectVector` _location _traceend _returnvalue))
  (bind _output_get_2 (set `self.hitActor` _hitactor))
  (`/Engine/EditorBlueprintResources/StandardMacros.IsValid` _output_get_2
    (:`Is Valid`
      (set `self.hitActorLoc` (`self.K2_GetActorLocation` _output_get_2)))
    (:`Is Not Valid`
      _))
  (`self.LerpToNewLoc`))

(fn `tryDamageHitActor`
  (`self.hitActor`
    (:`then`
      (if (< (`KismetMathLibrary.Vector_Distance` (`self.hitActorLoc`) (`self.K2_GetActorLocation` (`self.hitActor`))) (`self.dodgeableDistAfterTargetedToHit`))
        (message `/Game/Blueprints/Interactive/Destroyable/BPI_Destroyable.Damage` (`self.hitActor`) (`self.damageToDeal`) false "NewEnumerator5")))
    (:`else`)))

(fn `updateTrail`
  (`FXSystemComponent.SetVectorParameter` (`self.NS_EnemyMove`) "lastPos" (- (`self.prevLoc`) (`self.newLoc`)))
  (`ActorComponent.Activate` (`self.NS_EnemyMove`) false))

(fn `UserConstructionScript`)