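; BP_Save is a save game object that stores game settings as an array of Id/Value structs.
; Get and set functions search the array linearly by Id, and every change immediately writes the object to the "save" slot; reset clears the array.
; A missed lookup appends a zero-valued entry: get files it under "None" instead of the requested Id, and set drops the passed value.
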(fn `addSettingValue`
  (params (id :type Name))
  (`KismetArrayLibrary.Array_Add` (`self.settings`) (make `/Game/Blueprints/Settings/SSetting` id))
  (`GameplayStatics.SaveGameToSlot` self "save"))

(fn `getSettingValue`
  (params (id :type Name))
  (returns (value :type Integer))
  (for _array_element (`self.settings`)
    (bind (_id _value) (break `/Game/Blueprints/Settings/SSetting` _array_element))
    (if (== _id (`local.id`))
      (return _value)))
  (`self.addSettingValue` "None"))

(fn `resetSettings`
  (`KismetArrayLibrary.Array_Clear` (`self.settings`))
  (`GameplayStatics.SaveGameToSlot` self "save"))

(fn `setSettingValue`
  (params (id :type Name) (value :type Integer))
  (for (_array_element _array_index) (`self.settings`)
    (bind _id (break `/Game/Blueprints/Settings/SSetting` _array_element))
    (if (== _id (`local.id`))
      (`KismetArrayLibrary.Array_Set` (`self.settings`) _array_index (make `/Game/Blueprints/Settings/SSetting` _id (`local.value`)))
      (`GameplayStatics.SaveGameToSlot` self "save")
      (return)))
  (`self.addSettingValue` id)
  (return))