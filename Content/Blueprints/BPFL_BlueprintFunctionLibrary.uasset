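; Global helper function library for a VR rhythm game with enemies, exposing shared managers, level checks and color lookups.
; Manager getters route through the GameInstance, feeding wrappers that bind events to beats and control music tracks.
; Settings helpers use a single save slot and notify the VR pawn and post-process actor.
; Spatial helpers trace for floors and test-sweep child components to limit how far a hierarchy moves.
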(fn `bindEventToRhythm`
  (params (rhythm :type "/Game/Blueprints/Music/ERhythmSubscribe Enum" :default "NewEnumerator0") (Event :type "Delegate (by ref)"))
  (locals (beatMan :type "/Game/Blueprints/Music/BP_BeatManager Object Reference"))
  (bind _beatmanager (`self.getBeatManager` (`local.__WorldContext`)))
  (`/Engine/EditorBlueprintResources/StandardMacros.IsValid` _beatmanager
    (:`Is Valid`
      (set `local.beatMan` _beatmanager)
      (switch `/Game/Blueprints/Music/ERhythmSubscribe` (`local.rhythm`)
        (:`NewEnumerator0`
          (add `/Game/Blueprints/Music/BP_BeatManager.Bar` (`local.beatMan`) (`local.Event`)))
        (:`NewEnumerator1`
          (add `/Game/Blueprints/Music/BP_BeatManager.Beat` (`local.beatMan`) (`local.Event`)))
        (:`NewEnumerator2`
          (add `/Game/Blueprints/Music/BP_BeatManager.OffBeat` (`local.beatMan`) (`local.Event`)))
        (:`NewEnumerator3`
          (add `/Game/Blueprints/Music/BP_BeatManager.ErrorMarginStarted` (`local.beatMan`) (`local.Event`)))
        (:`NewEnumerator4`
          (add `/Game/Blueprints/Music/BP_BeatManager.ErrorMarginEnded` (`local.beatMan`) (`local.Event`)))
        (:`NewEnumerator5`
          (add `/Game/Blueprints/Music/BP_BeatManager.2Bar` (`local.beatMan`) (`local.Event`)))
        (:`NewEnumerator6`
          (add `/Game/Blueprints/Music/BP_BeatManager.4Bar` (`local.beatMan`) (`local.Event`)))))
    (:`Is Not Valid`
      (`KismetSystemLibrary.PrintString` null (`KismetStringLibrary.Concat_StrStr` "ERROR! Tried to bind event to " (`|GetEnumeratorNameAsString` (`local.rhythm`)) " too early :(") true true (struct :`R` 1.0 :`A` 1.0) 5.0))))

(fn `createSave`
  (returns (ReturnValue :type "/Game/Blueprints/BP_Save Object Reference"))
  (locals (newSave :type "/Game/Blueprints/BP_Save Object Reference"))
  (bind _returnvalue (`GameplayStatics.CreateSaveGameObject` "/Game/Blueprints/BP_Save.BP_Save_C"))
  (bind _output_get (set `local.newSave` _returnvalue))
  (`GameplayStatics.SaveGameToSlot` _output_get "save")
  (return (`local.newSave`)))

(fn `findFloor`
  (params (component :type "SceneComponent Object Reference") (checkDist :type "Float (double-precision)" :default 10.0) (maxAngleToConsiderFloor :type "Float (double-precision)" :default 45.0))
  (returns (floor :type "Actor Object Reference") (hitLocation :type "Vector Structure"))
  (bind _returnvalue (`SceneComponent.K2_GetComponentLocation` component))
  (bind _maxangletoconsiderfloor (`local.maxAngleToConsiderFloor`))
  (bind (_x _y _z) (`KismetMathLibrary.BreakVector3f` _returnvalue))
  (bind (_outhit _returnvalue_2) (`KismetSystemLibrary.LineTraceSingle` (`local.__WorldContext`) _returnvalue (`KismetMathLibrary.MakeVector` _x _y (- _z (`local.checkDist`))) "TraceTypeQuery1" false (`|MakeArray` (`ActorComponent.GetOwner` component))))
  (if _returnvalue_2
    (bind (_bblockinghit _binitialoverlap _time _distance _location _impactpoint _normal _impactnormal _physmat _hitactor) (`GameplayStatics.BreakHitResult` _outhit))
    (bind (_outslopepitchdegreeangle _outsloperolldegreeangle) (`KismetMathLibrary.GetSlopeDegreeAngles` (`SceneComponent.GetRightVector` (`local.component`)) _normal (`KismetMathLibrary.MakeVector` 0.0 0.0 1.0)))
    (if (`KismetMathLibrary.BooleanNOR` (> (`KismetMathLibrary.Abs` _outslopepitchdegreeangle) _maxangletoconsiderfloor) (> (`KismetMathLibrary.Abs` _outsloperolldegreeangle) _maxangletoconsiderfloor))
      (return _hitactor _location)
      (else
        _)))
  (return null (0.0 0.0 0.0)))

(fn `findFloorActor`
  (params (actor :type "Actor Object Reference") (checkDist :type "Float (double-precision)" :default 10.0) (maxAngleToConsiderFloor :type "Float (double-precision)" :default 45.0))
  (returns (floor :type "Actor Object Reference") (hitLocation :type "Vector Structure"))
  (bind (_floor _hitlocation) (`self.findFloor` (`Actor.RootComponent` actor) checkDist maxAngleToConsiderFloor (`local.__WorldContext`)))
  (return _floor _hitlocation))

(fn `getAIHivemind`
  (returns (hivemind :type "/Game/Blueprints/Enemies/BP_AIHivemind Object Reference"))
  (return (`/Game/Blueprints/GI_GameInstance.aiHivemind` (`self.getGI` (`local.__WorldContext`)))))

(fn `getBeatManager`
  (returns (beatManager :type "/Game/Blueprints/Music/BP_BeatManager Object Reference"))
  (return (`/Game/Blueprints/GI_GameInstance.beatManager` (`self.getGI` (`local.__WorldContext`)))))

(fn `getBeatStartDelay`
  (params (isBeatBindEventDelay :type Boolean :default true))
  (returns (delay :type "Float (double-precision)"))
  (bind (_bindbeateventsstartdelay _beatmanagerstartdelay) (`/Game/Blueprints/GI_GameInstance.getDelays` (`self.getGI` (`local.__WorldContext`))))
  (return (`KismetMathLibrary.SelectFloat` _bindbeateventsstartdelay _beatmanagerstartdelay (`local.isBeatBindEventDelay`))))

(fn `getGI`
  (returns (GI :type "/Game/Blueprints/GI_GameInstance Object Reference"))
  (return (cast `/Game/Blueprints/GI_GameInstance` (`GameplayStatics.GetGameInstance` (`local.__WorldContext`)) :!pure true)))

(fn `getMainColor`
  (params (isColorSecondary :type Boolean))
  (returns (color :type "LinearColor Structure"))
  (bind _returnvalue (`KismetMaterialLibrary.GetVectorParameterValue` (`local.__WorldContext`) "/Game/Materials/_MPC/MPC_Colors.MPC_Colors" (select `bool` isColorSecondary :`false` "ColorPrimary" :`true` "ColorSecondary" :!type "Name")))
  (return _returnvalue))

(fn `getSave`
  (returns (ReturnValue :type "/Game/Blueprints/BP_Save Object Reference"))
  (bind _returnvalue (`GameplayStatics.DoesSaveGameExist` "save"))
  (if _returnvalue
    (bind _returnvalue_2 (`GameplayStatics.LoadGameFromSlot` "save"))
    (return (cast `/Game/Blueprints/BP_Save` _returnvalue_2 :!pure true))
    (else
      (bind _returnvalue_3 (`self.createSave` (`local.__WorldContext`)))
      (return _returnvalue_3))))

(fn `getSavedSetting`
  (params (id :type Name))
  (returns (value :type Integer))
  (return (`/Game/Blueprints/BP_Save.getSettingValue` (`self.getSave` (`local.__WorldContext`)) id)))

(fn `getTrackManager`
  (returns (trackManager :type "/Game/Blueprints/Music/BPC_TrackManager Object Reference"))
  (return (`/Game/Blueprints/Music/BP_BeatManager.BPC_TrackManager` (`self.getBeatManager` (`local.__WorldContext`)))))

(fn `getWaveSpawner`
  (returns (spawner :type "/Game/Blueprints/Enemies/Waves/BP_EnemyWaveSpawner Object Reference"))
  (return (`/Game/Blueprints/GI_GameInstance.activeSpawner` (`self.getGI` (`local.__WorldContext`)))))

(fn `groundVector`
  (params (inPosition :type "Vector Structure") (checkHeight :type "Float (double-precision)" :default 3000.0))
  (returns (groundedPosition :type "Vector Structure") (foundGround :type Boolean))
  (bind (_inposition_x _inposition_y) (`KismetMathLibrary.BreakVector` (`local.inPosition`)))
  (bind (_outhit _returnvalue) (`KismetSystemLibrary.LineTraceSingle` (`local.__WorldContext`) inPosition (- inPosition (`KismetMathLibrary.MakeVector` 0.0 0.0 checkHeight)) "TraceTypeQuery1"))
  (if _returnvalue
    (return (`KismetMathLibrary.MakeVector` _inposition_x _inposition_y (`.Z` (`KismetMathLibrary.BreakVector3f` (`.Location` (`GameplayStatics.BreakHitResult` _outhit))))) true)
    (else
      (return (`local.inPosition`) false))))

(fn `isActorAnEnemy`
  (params (actor :type "Actor Object Reference"))
  (returns (result :type Boolean))
  (return (`KismetMathLibrary.ClassIsChildOf` (`GameplayStatics.GetObjectClass` actor) "/Game/Blueprints/Enemies/BP_EnemyBase.BP_EnemyBase_C")))

(fn `isCurrentlyInErrorMargin`
  (returns (inErrorMargin :type Boolean))
  (return (`/Game/Blueprints/Music/BP_BeatManager.checkInErrorMargin` (`self.getBeatManager` (`local.__WorldContext`)))))

(fn `isInLevel`
  (params (levelName :type String))
  (returns (return :type Boolean))
  (bind _returnvalue (`GameplayStatics.GetCurrentLevelName` (`local.__WorldContext`)))
  (return (`KismetStringLibrary.EqualEqual_StrStr` _returnvalue levelName)))

(fn `isInMenu`
  (returns (return :type Boolean))
  (for _array_element (`|MakeArray` "Menu" "Warning" "Settings")
    (if (`self.isInLevel` _array_element (`local.__WorldContext`))
      (return true)))
  (return false))

(fn `isOnGoToMenuScreen`
  (returns (return :type Boolean))
  (return (`self.isInLevel` "Warning" (`local.__WorldContext`))))

(fn `isThereActorOfClass`
  (params (ActorClass :type "Actor Class Reference"))
  (returns (ReturnValue :type Boolean))
  (bind _returnvalue (`GameplayStatics.GetActorOfClass` (`local.__WorldContext`) ActorClass))
  (return (`KismetSystemLibrary.IsValid` _returnvalue)))

(fn `refreshMusicTracks`
  (`/Game/Blueprints/Music/BPC_TrackManager.tryPlayEverything` (`/Game/Blueprints/Music/BP_BeatManager.BPC_TrackManager` (`self.getBeatManager` (`local.__WorldContext`)))))

(fn `resetSettings`
  (`|ExecutionSequence`
    (:`then_0`
      (`/Game/Blueprints/BP_Save.resetSettings` (`self.getSave` (`local.__WorldContext`)))
      (bind _outactors (`GameplayStatics.GetAllActorsOfClass` (`local.__WorldContext`) "/Game/Blueprints/Interactive/MiscInteractives/BP_SettingSetter.BP_SettingSetter_C"))
      (for _array_element _outactors
        (`/Game/Blueprints/Interactive/MiscInteractives/BP_SettingSetter.setNewSettingValue` _array_element 0 false)))
    (:`then_1`
      (`self.sendNewSettingUpdates` (`local.__WorldContext`)))))

(fn `sendNewSettingUpdates`
  (`|ExecutionSequence`
    (:`then_0`
      (bind _asvrpawn (cast `/Game/VRTemplate/Blueprints/VRPawn` (`GameplayStatics.GetPlayerPawn` (`local.__WorldContext`))))
      (`/Game/VRTemplate/Blueprints/VRPawn.updateSettings` _asvrpawn))
    (:`then_1`
      (bind _returnvalue (`GameplayStatics.GetActorOfClass` (`local.__WorldContext`) "/Game/Blueprints/PostColors/BP_PostProcess.BP_PostProcess_C"))
      (`/Game/Blueprints/PostColors/BP_PostProcess.UpdateSettings` _returnvalue))))

(fn `setElectricityColor`
  (params (particles :type "NiagaraComponent Object Reference") (intensityModifier :type "Float (double-precision)" :default 1.0))
  (`NiagaraComponent.SetVariableLinearColor` (`local.particles`) "ElectricityColor" (* (`KismetMathLibrary.Conv_DoubleToLinearColor` (`local.intensityModifier`)) (`self.getMainColor` false (`local.__WorldContext`)))) ; Use electricity color
)

(fn `setLocationWithSweepHierarchy`
  (params (root :type "SceneComponent Object Reference") (transform :type "Transform Structure"))
  (returns (percentTraveled :type "Float (double-precision)"))
  (locals (rootSaved :type "SceneComponent Object Reference") (transformSaved :type "Transform Structure") (distance :type "Float (double-precision)" :default 0.0))
  (`/Engine/EditorBlueprintResources/StandardMacros.IsValid` root
    (:`Is Valid`
      (`|ExecutionSequence`
        (:`then_0`
          (set `local.rootSaved` root)
          (set `local.transformSaved` transform))
        (:`then_1`
          ;[1 1 1] Move root by shortest distance
          (set `local.distance` (`self.sweepHierarchy` (`local.rootSaved`) (`local.transformSaved`) (`local.__WorldContext`)))
          (`|ExecutionSequence`
            (:`then_0`
              (bind _rootsaved (`local.rootSaved`)
                (:`then`
                  (`SceneComponent.K2_SetWorldLocationAndRotation` _rootsaved (.location (`KismetMathLibrary.TLerp` (`SceneComponent.K2_GetComponentToWorld` (`local.rootSaved`)) (`local.transformSaved`) (`local.distance`))) (.rotation (`KismetMathLibrary.TLerp` (`SceneComponent.K2_GetComponentToWorld` (`local.rootSaved`)) (`local.transformSaved`) (`local.distance`))) false true))
                (:`else`)))
            (:`then_1`
              (return (`local.distance`)))))))))

(fn `setSave`
  (params (SaveGameObject :type "SaveGame Object Reference"))
  (returns (ReturnValue :type Boolean))
  (bind _returnvalue (`GameplayStatics.SaveGameToSlot` SaveGameObject "save"))
  (return _returnvalue))

(fn `setSavedSetting`
  (params (id :type Name) (value :type Integer) (sendUpdate :type Boolean :default true))
  (`/Game/Blueprints/BP_Save.setSettingValue` (`self.getSave` (`local.__WorldContext`)) id value)
  (if (`local.sendUpdate`)
    (`self.sendNewSettingUpdates` (`local.__WorldContext`))))

(fn `sweepHierarchy`
  (params (root :type "SceneComponent Object Reference") (transform :type "Transform Structure"))
  (returns (dist :type "Float (double-precision)"))
  (locals (distance :type "Float (double-precision)" :default 1.0) (rootSaved :type "SceneComponent Object Reference") (transformSaved :type "Transform Structure") (storedTransform :type "Transform Structure"))
  (`|ExecutionSequence`
    (:`then_0`
      (set `local.rootSaved` root)
      (set `local.transformSaved` transform))
    (:`then_1`
      ;[1 1 1] Move each child, store shortest distance then move child back
      (for _array_element (`SceneComponent.GetChildrenComponents` (`local.rootSaved`) true)
        (`/Engine/EditorBlueprintResources/StandardMacros.IsValid` _array_element
          (:`Is Valid`
            (bind _returnvalue (`SceneComponent.K2_GetComponentToWorld` _array_element))
            (set `local.storedTransform` _returnvalue)
            (bind _sweephitresult (`SceneComponent.K2_SetWorldLocationAndRotation` _array_element (.location (`KismetMathLibrary.ComposeTransforms` (`KismetMathLibrary.ComposeTransforms` _returnvalue (`KismetMathLibrary.InvertTransform` (`SceneComponent.K2_GetComponentToWorld` (`local.rootSaved`)))) (`local.transformSaved`))) (.rotation (`KismetMathLibrary.ComposeTransforms` (`KismetMathLibrary.ComposeTransforms` _returnvalue (`KismetMathLibrary.InvertTransform` (`SceneComponent.K2_GetComponentToWorld` (`local.rootSaved`)))) (`local.transformSaved`))) true true))
            (set `local.distance` (`KismetMathLibrary.FMin` (`local.distance`) (`.Time` (`GameplayStatics.BreakHitResult` _sweephitresult))))
            (`SceneComponent.K2_SetWorldLocationAndRotation` _array_element (.location (`local.storedTransform`)) (.rotation (`local.storedTransform`)) false true))))
      (return (`local.distance`)))))

(fn `tryPlayTrackByCondition`
  (params (condition :type "/Game/Blueprints/Music/Music/EPlayCondition Enum" :default "NewEnumerator0") (allNotJustFirst :type Boolean) (ignoreCondition :type Boolean))
  (`/Game/Blueprints/Music/BPC_TrackManager.trySetTrackPlayingByCondition` (`/Game/Blueprints/Music/BP_BeatManager.BPC_TrackManager` (`self.getBeatManager` (`local.__WorldContext`))) condition allNotJustFirst ignoreCondition))