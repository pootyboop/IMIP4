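; Music beat manager that runs a Quartz clock and broadcasts bar, beat, off-beat and error-margin events, registering itself on the game instance.
; Setup reads BPM and tracks from DT_MusicLevels, adding universal tracks for BPCTrackManager, unless overridden for debug audio.
; Subdivision ticks counted from each beat open and close a timing window around it.
; Beats can pulse MPC_Colors and post-process; bar counts trigger quantized loop requeue and transport reset.
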(event `self.ReceiveBeginPlay`
  (`self.updateGIRef`)
  (set `/Game/Blueprints/Music/BPC_TrackManager.forceMute` (`self.forceMute`) (`self.BPC_TrackManager`))
  (`KismetSystemLibrary.K2_SetTimerDelegate` (delegate `StartQuartz`) (`/Game/Blueprints/BPFL_BlueprintFunctionLibrary.getBeatStartDelay` false)))

(event `StartQuartz`
  (`self.setQuartzState` "NewEnumerator0"))

(event `QueueMusic`
  ;[1 1 1] Queue Next Loop
  (bind _debugmusic (`self.debugMusic`)
    (:`then`
      (bind _returnvalue (`GameplayStatics.CreateSound2D` (select `bool` (`self.overrideMusicLevelInfo`) :`false` "/Game/Audio/Silent.Silent" :`true` _debugmusic) 1.0 1.0 0.0 null))
      (`AudioComponent.PlayQuantized` _returnvalue (`self.quartzClock`) (make `QuartzQuantizationBoundary` (`self.barQuantizationBoundary`) 1.0 "CurrentTimeRelative") (delegate `QuantizedMusic`) 0.0 0.0 1.0 "Linear"))
    (:`else`)))

(event `QuantizedMusic`
  (params (EventType :type "EQuartzCommandDelegateSubType Enum" :default "CommandOnFailedToQueue") (Name :type Name))
  ;[1 1 1] Queue Next Loop
  (switch `EQuartzCommandDelegateSubType` EventType
    (:`CommandOnQueued`
      (`/Engine/EditorBlueprintResources/StandardMacros.DoOnce` false
        (:`Completed`
          (`QuartzClockHandle.StartClock` (`self.quartzClock`)))))))

(event `BarEvents`
  (params (ClockName :type Name) (QuantizationType :type "EQuartzCommandQuantization Enum" :default "Bar") (NumBars :type Integer) (Beat :type Integer) (BeatFraction :type "Float (single-precision)"))
  ;[1 1 1] Track Bars + Loop
  (`|ExecutionSequence`
    (:`then_0`
      (`self.onBar` Beat NumBars))
    (:`then_1`
      (`self.Bar`))))

(event `BeatEvents`
  (params (ClockName :type Name) (QuantizationType :type "EQuartzCommandQuantization Enum" :default "Bar") (NumBars :type Integer) (Beat :type Integer) (BeatFraction :type "Float (single-precision)"))
  ;[1 1 1] Track Beats
  (`|ExecutionSequence`
    (:`then_0`
      (`self.onBeat` Beat))
    (:`then_1`
      (`self.Beat`))
    (:`then_2`
      (if (`self.isOnOff-Beat`)
        (`self.OffBeat`)))))

(event `ErrorMarginEvents`
  (params (ClockName :type Name) (QuantizationType :type "EQuartzCommandQuantization Enum" :default "Bar") (NumBars :type Integer) (Beat :type Integer) (BeatFraction :type "Float (single-precision)"))
  ;[1 1 1] Error Margin
  (`self.updateErrorMargin`))

(event `BeatIntensityFade`
  ;[1 1 1] Fade MPC by beats
  (`TimelineComponent.SetPlayRate` (`self.BeatIntensity`) (/ (/ (`self.BPM`) 60.0) (select `EQuartzCommandQuantization` (`self.beatQuantizationBoundary`) :`ThirtySecondNote` 0.125 :`SixteenthNote` 0.25 :`EighthNote` 0.5 :`QuarterNote` 1.0 :`HalfNote` 2.0 :`WholeNote` 4.0)))
  (`KismetMaterialLibrary.SetVectorParameterValue` "/Game/Materials/_MPC/MPC_Colors.MPC_Colors" "BeatColor" (`/Game/Blueprints/BPFL_BlueprintFunctionLibrary.getMainColor` (`self.isOnOff-Beat`)))
  (bind (_direction _beatintensity) (`Timeline|BeatIntensity` :!via `PlayFromStart`)
    (:`Update`
      (`KismetMaterialLibrary.SetScalarParameterValue` "/Game/Materials/_MPC/MPC_Colors.MPC_Colors" "BeatIntensity" _beatintensity)
      (bind _postprocess (`self.postProcess`)
        (:`then`
          (message `/Game/Blueprints/Music/BeatSync/BPI_BeatSync.OnBeatIntensityFadeUpdate` _postprocess _beatintensity (`self.isOnOff-Beat`)))
        (:`else`)))))

(fn `applyRhythm`
  (params (rhythmObject :type "/Game/Blueprints/Music/Music/Rhythms/BP_RhythmBase Object Reference")))

(fn `checkInErrorMargin`
  (returns (inErrorMargin :type Boolean))
  (return (`self.inErrorMargin`)))

(fn `environmentBeat`
  (if (`self.affectEnvironment`)
    (`self.BeatIntensityFade`)
    (if (`self.overrideMusicLevelInfo`)
      (bind _debugbeatsound (`self.debugBeatSound`)
        (:`then`
          (`GameplayStatics.PlaySound2D` _debugbeatsound 1.0 1.0 0.0 null null))
        (:`else`)))))

(fn `getErrorMarginAsInt`
  (params (errorMarginAsString :type String :default "1/32"))
  (returns (ReturnValue :type Integer))
  (return (/ (`KismetStringLibrary.Conv_StringToInt` (`KismetStringLibrary.Replace` errorMarginAsString "1/")) (`self.numOfBeatsInBar`))))

(fn `getMusicLevelByName`
  (params (RowName :type Name :default "UNIVERSAL"))
  (returns (data :type "/Game/Blueprints/Music/Music/SMusic Structure"))
  (bind _returnvalue (`|GetDataTableRow` "/Game/Blueprints/Music/Music/DT_MusicLevels.DT_MusicLevels" RowName)
    (:`then`
      (return _returnvalue))))

(fn `onBar`
  (params (beat :type Integer) (numBars :type Integer))
  (bind _returnvalue (`KismetMathLibrary.SelectInt` beat numBars (`self.repeatByBeats`)))
  (`|ExecutionSequence`
    (:`then_0`
      (`/Engine/EditorBlueprintResources/StandardMacros.FlipFlop`
        (:`A`
          (`self.2Bar`))))
    (:`then_1`
      (if (`self.printBeatInformation`)
        (`KismetSystemLibrary.PrintString` (`KismetStringLibrary.Concat_StrStr` "Bar " (`KismetStringLibrary.Conv_IntToString` _returnvalue)) true true (struct :`R` 1.0 :`A` 1.0)))
      (if (== _returnvalue (`self.numToLoop`))
        (`self.QueueMusic`)
        (`QuartzClockHandle.ResetTransportQuantized` :`self` (`self.quartzClock`) :`InQuantizationBoundary` (make `QuartzQuantizationBoundary` (`self.barQuantizationBoundary`) 1.0 "CurrentTimeRelative"))))))

(fn `onBeat`
  (params (beat :type Integer))
  (set `self.errorMarginCounter` 0) ; Reset error margin counter each beat
  (set `self.isOnOff-Beat` (and (== (mod beat 2) 0) (!= beat 0)))
  (`self.environmentBeat`)
  (if (`self.printBeatInformation`)
    (`KismetSystemLibrary.PrintString` (`KismetStringLibrary.Concat_StrStr` "Beat " (`KismetStringLibrary.Conv_IntToString` beat)) true true (struct :`G` 0.254361 :`B` 1.0 :`A` 1.0))))

(fn `setQuartzState`
  (params (newState :type "/Game/Blueprints/Music/EQuartzState Enum" :default "NewEnumerator0"))
  (bind _output_get (set `self.quartzState` newState))
  (switch `/Game/Blueprints/Music/EQuartzState` _output_get
    (:`NewEnumerator0`
      (bind _quartzclock (`self.quartzClock`)
        (:`then`
          (`QuartzClockHandle.ResumeClock` _quartzclock))
        (:`else`
          (`self.setupQuartz`))))
    (:`NewEnumerator1`
      (bind _quartzclock_2 (`self.quartzClock`)
        (:`then`
          (`QuartzClockHandle.PauseClock` _quartzclock_2))
        (:`else`)))
    (:`NewEnumerator2`
      (bind _quartzclock_3 (`self.quartzClock`)
        (:`then`
          (`QuartzClockHandle.StopClock` _quartzclock_3 true)
          (set `self.quartzClock` null))
        (:`else`)))))

(fn `setupEnvironmentBeat`
  (if (`self.affectEnvironment`)
    (bind _returnvalue (`GameplayStatics.GetActorOfClass` "/Game/Blueprints/PostColors/BP_PostProcess.BP_PostProcess_C"))
    (set `self.postProcess` _returnvalue)))

(fn `setupMusicLevel`
  (params (lvlName :type Name))
  (returns (tracksForLevel :type "Array of /Game/Blueprints/Music/Music/SMusicTrack Structure") (success :type Boolean))
  (locals (allTracks :type "Array of /Game/Blueprints/Music/Music/SMusicTrack Structure") (lvlData :type "/Game/Blueprints/Music/Music/SMusic Structure"))
  (bind (_bpm _rhythm _tracks) (break `/Game/Blueprints/Music/Music/SMusic` (`local.lvlData`)))
  (bind (_bpm_2 _rhythm_2 _tracks_2) (break `/Game/Blueprints/Music/Music/SMusic` (`self.getMusicLevelByName` "UNIVERSAL")))
  (set `local.lvlData` (`self.getMusicLevelByName` (`local.lvlName`)))
  (if (and (not (`self.overrideMusicLevelInfo`)) (`KismetArrayLibrary.Array_IsNotEmpty` (`.tracks_13_22464ED4425D37874EEB6D8F47206DF7` (break `/Game/Blueprints/Music/Music/SMusic` (`local.lvlData`)))))
    (set `self.BPM` _bpm)
    (`self.applyRhythm` _rhythm)
    (bind _output_get (set `local.allTracks` _tracks))
    (if (`KismetArrayLibrary.Array_IsNotEmpty` _tracks_2)
      (`KismetArrayLibrary.Array_Append` _output_get _tracks_2))
    (return (`local.allTracks`) true)
    (else
      (return _ false))))

(fn `setupQuartz`
  (locals (success :type Boolean :default false) (tracksForLevel :type "Array of /Game/Blueprints/Music/Music/SMusicTrack Structure"))
  (bind (_tracksforlevel _success) (`self.setupMusicLevel` (`self.musicLvlID`)))
  (set `local.tracksForLevel` _tracksforlevel)
  (set `local.success` _success)
  (bind _returnvalue (`QuartzSubsystem.CreateNewClock` (subsystem `QuartzSubsystem`) (`self.clockName`) (make `QuartzClockSettings` (make `QuartzTimeSignature` (`self.numOfBeatsInBar`))) false true))
  (bind _output_get (set `self.quartzClock` _returnvalue))
  (bind _clockhandle (`QuartzClockHandle.SetBeatsPerMinute` :`self` _output_get :`BeatsPerMinute` (`self.BPM`)))
  (bind _clockhandle_2 (`QuartzClockHandle.SubscribeToQuantizationEvent` _clockhandle (`self.barQuantizationBoundary`) (`|CreateDelegate` :!event `BarEvents`)))
  (bind _clockhandle_3 (`QuartzClockHandle.SubscribeToQuantizationEvent` _clockhandle_2 (`self.beatQuantizationBoundary`) (`|CreateDelegate` :!event `BeatEvents`)))
  (bind _clockhandle_4 (`QuartzClockHandle.SubscribeToQuantizationEvent` _clockhandle_3 (`self.errorMarginQuantizationBoundary`) (`|CreateDelegate` :!event `ErrorMarginEvents`)))
  (set `self.quartzClock` _clockhandle_4)
  (set `self.errorMarginInt` (`self.getErrorMarginAsInt` "1/32"))
  (if (`local.success`)
    (`/Game/Blueprints/Music/BPC_TrackManager.setAvailableTracks` (`self.BPC_TrackManager`) (`local.tracksForLevel`)))
  (`self.setupEnvironmentBeat`)
  (`self.QueueMusic`))

(fn `updateErrorMargin`
  (`/Engine/EditorBlueprintResources/StandardMacros.IncrementInt` (`self.errorMarginCounter`)
    (:`  `
      (if (and (== (`self.errorMarginCounter`) 2) (`self.inErrorMargin`))
        (set `self.inErrorMargin` false)
        (`self.ErrorMarginEnded`)
        (if (`self.printBeatInformation`)
          (`KismetSystemLibrary.PrintString` "Error Margin End" true true (struct :`R` 1.0 :`G` 0.431373 :`A` 1.0)))
        (elif (and (== (`self.errorMarginCounter`) (- (`self.errorMarginInt`) 1)) (not (`self.inErrorMargin`)))
          (set `self.inErrorMargin` true)
          (`self.ErrorMarginStarted`)
          (if (`self.printBeatInformation`)
            (`KismetSystemLibrary.PrintString` "Error Margin Start" true true (struct :`R` 1.0 :`G` 0.431373 :`A` 1.0))))))))

(fn `updateGIRef`
  (set `/Game/Blueprints/GI_GameInstance.beatManager` self (`/Game/Blueprints/BPFL_BlueprintFunctionLibrary.getGI`)))

(fn `UserConstructionScript`)