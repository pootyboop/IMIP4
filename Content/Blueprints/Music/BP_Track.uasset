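; Music track actor that plays the audio from its TrackData and replays it on a rhythm set by the track's length.
; Each loop either decrements a loop counter and replays, or, at -1, replays only if the track manager reports the track's condition met.
; It destroys itself when audio finishes with the counter at zero, and reports its ID to the track manager on EndPlay.
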(event `self.ReceiveBeginPlay`
  (bind (_id _audio _condition _length _loopsafterconditionmet) (break `/Game/Blueprints/Music/Music/SMusicTrack` (`self.trackData`)))
  (`AudioComponent.SetSound` (`self.Audio`) _audio)
  (set `self.loopsAfterConditionMet` _loopsafterconditionmet)
  (`self.Play Track`)
  (`/Game/Blueprints/BPFL_BlueprintFunctionLibrary.bindEventToRhythm` _length (delegate `OnLoop`)))

(event `OnLoop`
  (bind _loopsafterconditionmet (`self.loopsAfterConditionMet`))
  (switch `int` _loopsafterconditionmet
    (:`Default`
      (`/Engine/EditorBlueprintResources/StandardMacros.DecrementInt` _loopsafterconditionmet
        (:`  `
          (`self.Play Track` :!label _label))))
    (:`-1`
      (if (`/Game/Blueprints/Music/BPC_TrackManager.isConditionMet` (`/Game/Blueprints/BPFL_BlueprintFunctionLibrary.getTrackManager`) (`.condition_7_65A08FB2466D53BA207E45834E8741BC` (break `/Game/Blueprints/Music/Music/SMusicTrack` (`self.trackData`))))
        (goto _label)))
    (:`0`)))

(event `Play Track`
  (`AudioComponent.Play` (`self.Audio`) 0.0)
  (if (`self.printDebug`)
    (`KismetSystemLibrary.PrintString` (`KismetStringLibrary.Concat_StrStr` "Play " (`KismetStringLibrary.Conv_NameToString` (`.ID_18_60563C7A4D6EEF72504C398F2BBB4B10` (break `/Game/Blueprints/Music/Music/SMusicTrack` (`self.trackData`))))) true true (struct :`R` 0.388978 :`B` 1.0 :`A` 1.0))))

(event `self.Audio.OnAudioFinished`
  (if (== (`self.loopsAfterConditionMet`) 0)
    (`self.K2_DestroyActor`)))

(event `self.ReceiveEndPlay`
  (params (EndPlayReason :type "EEndPlayReason Enum" :default "Destroyed"))
  (bind _trackdata_id (break `/Game/Blueprints/Music/Music/SMusicTrack` (`self.trackData`)))
  (`/Game/Blueprints/Music/BPC_TrackManager.onTrackDestroyed` (`/Game/Blueprints/BPFL_BlueprintFunctionLibrary.getTrackManager`) _trackdata_id))

(fn `UserConstructionScript`)