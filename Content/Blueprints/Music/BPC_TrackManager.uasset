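; Music component that starts tracks to match gameplay conditions such as enemy counts, living enemy types and active liquid, electricity or electrocution actors.
; Setting available tracks destroys those playing, then spawns a BP_Track actor for each eligible one, stored by ID to prevent duplicates.
; Outside calls can trigger tracks by condition, optionally bypassing checks, while ForceMute blocks new starts.
; Enemy conditions query the wave spawner; the enemy-attacking condition always returns false.
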(fn `enemyTypeAlive`
  (params (enemyType :type "/Game/Blueprints/Enemies/_EnemyTypes/EEnemyType Enum" :default "NewEnumerator0"))
  (returns (ReturnValue :type Boolean))
  (bind _spawner (`/Game/Blueprints/BPFL_BlueprintFunctionLibrary.getWaveSpawner`))
  (`/Engine/EditorBlueprintResources/StandardMacros.IsValid` _spawner
    (:`Is Valid`
      (return (> (`/Game/Blueprints/Enemies/Waves/BP_EnemyWaveSpawner.getEnemyTypeCt` _spawner enemyType) 0)))
    (:`Is Not Valid`
      (return false))))

(fn `getEnemyCt`
  (params (ct :type Integer :default 1))
  (returns (enemyCount :type Integer) (ReturnValue :type Boolean))
  (bind _spawner (`/Game/Blueprints/BPFL_BlueprintFunctionLibrary.getWaveSpawner`))
  (bind _enemycount (`/Game/Blueprints/Enemies/Waves/BP_EnemyWaveSpawner.enemyCount` _spawner))
  (`/Engine/EditorBlueprintResources/StandardMacros.IsValid` _spawner
    (:`Is Valid`
      (return _enemycount (>= _enemycount ct)))
    (:`Is Not Valid`
      (return 0 (>= 0 ct)))))

(fn `isConditionMet`
  (params (condition :type "/Game/Blueprints/Music/Music/EPlayCondition Enum" :default "NewEnumerator0"))
  (returns (isMet :type Boolean))
  (`|ExecutionSequence`
    (:`then_0`
      (switch `/Game/Blueprints/Music/Music/EPlayCondition` condition
        (:`NewEnumerator0`
          (return true))
        (:`NewEnumerator4`
          (return (`/Game/Blueprints/BPFL_BlueprintFunctionLibrary.isThereActorOfClass` "/Game/Blueprints/Player/LiquidGlob/BP_LiquidGlob.BP_LiquidGlob_C")))
        (:`NewEnumerator5`
          (return (`/Game/Blueprints/BPFL_BlueprintFunctionLibrary.isThereActorOfClass` "/Game/Blueprints/Player/Electricity/BP_ElectricityChainer.BP_ElectricityChainer_C")))
        (:`NewEnumerator1`
          (return (`/Game/Blueprints/BPFL_BlueprintFunctionLibrary.isThereActorOfClass` "/Game/Blueprints/Interactive/MiscInteractives/BP_Electrocution.BP_Electrocution_C")))
        (:`NewEnumerator9`
          (return false))
        (:`NewEnumerator11`
          ;[1 0.1294 0] Enemy Counts
          (return (not (`.ReturnValue` (`self.getEnemyCt` 1)))))
        (:`NewEnumerator2`
          (return (`.ReturnValue` (`self.getEnemyCt` 1))))
        (:`NewEnumerator10`
          (return (`.ReturnValue` (`self.getEnemyCt` 2))))
        (:`NewEnumerator3`
          (return (`.ReturnValue` (`self.getEnemyCt` 3))))
        (:`NewEnumerator6`
          ;[1 0 0] Enemy Types
          (return (`self.enemyTypeAlive` "NewEnumerator0")))
        (:`NewEnumerator7`
          (return (`self.enemyTypeAlive` "NewEnumerator1")))
        (:`NewEnumerator8`
          (return (`self.enemyTypeAlive` "NewEnumerator2")))
        (:`NewEnumerator12`
          (return (`self.enemyTypeAlive` "NewEnumerator3")))
        (:`NewEnumerator13`
          (return (`self.enemyTypeAlive` "NewEnumerator4")))))
    (:`then_1`
      (return false) ; No logic, assume not met
    )))

(fn `isTrackPlaying`
  (params (ID :type "Name (by ref)"))
  (returns (ReturnValue :type Boolean))
  (return (`.ReturnValue` (`BlueprintMapLibrary.Map_Find` (`self.playing`) ID))))

(fn `onTrackDestroyed`
  (params (ID :type Name))
  (`BlueprintMapLibrary.Map_Remove` (`self.playing`) ID))

(fn `setAvailableTracks`
  (params (availableTracks :type "Array of /Game/Blueprints/Music/Music/SMusicTrack Structure"))
  (`|ExecutionSequence`
    (:`then_0`
      (bind _values (`BlueprintMapLibrary.Map_Values` (`self.playing`)))
      (for _array_element _values
        (`Actor.K2_DestroyActor` _array_element))
      (`BlueprintMapLibrary.Map_Clear` (`self.playing`)))
    (:`then_1`
      (set `self.availableTracks` availableTracks)
      (`self.tryPlayEverything`))))

(fn `tryPlayEverything`
  (for _array_element (`self.availableTracks`)
    (`self.trySetTrackPlaying` _array_element)))

(fn `trySetTrackPlaying`
  (params (track :type "/Game/Blueprints/Music/Music/SMusicTrack Structure") (ignoreCondition :type Boolean))
  (returns (success :type Boolean))
  (bind (_id _audio _condition) (break `/Game/Blueprints/Music/Music/SMusicTrack` track))
  (if (not (`self.forceMute`))
    (if (and (not (`self.isTrackPlaying` _id)) (or (`local.ignoreCondition`) (`self.isConditionMet` _condition)))
      (bind _returnvalue (`|SpawnActorFromClass` "/Game/Blueprints/Music/BP_Track.BP_Track_C" (`KismetMathLibrary.MakeTransform` (0.0 0.0 0.0)) "Undefined" "MultiplyWithRoot" null (`local.track`) null))
      (`BlueprintMapLibrary.Map_Add` (`self.playing`) (`.ID_18_60563C7A4D6EEF72504C398F2BBB4B10` (break `/Game/Blueprints/Music/Music/SMusicTrack` (`local.track`))) _returnvalue)
      (return true)
      (else
        (return false)))
    (else
      (return false))))

(fn `trySetTrackPlayingByCondition`
  (params (condition :type "/Game/Blueprints/Music/Music/EPlayCondition Enum" :default "NewEnumerator0") (allNotJustFirst :type Boolean) (ignoreCondition :type Boolean))
  (returns (success :type Boolean))
  (locals (playedTrack :type Boolean :default false))
  (for _array_element (`self.availableTracks`)
    (if (`|EnumEquality` condition (`.condition_7_65A08FB2466D53BA207E45834E8741BC` (break `/Game/Blueprints/Music/Music/SMusicTrack` _array_element)))
      (bind _success (`self.trySetTrackPlaying` _array_element (`local.ignoreCondition`)))
      (set `local.playedTrack` _success)
      (if (`local.allNotJustFirst`)
        (return (`local.playedTrack`)))))
  (return (`local.playedTrack`)))