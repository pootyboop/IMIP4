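; BP_AimAssister is an actor that sticks to a target's interaction point, apparently to assist the player's aim.
; SetTarget stores the target and picks a component to follow: the one from GetInteractionTransformMessage, falling back to the root component, or none if the target is invalid.
; Each Tick it moves to that component's world location with a swept move.
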(event `self.ReceiveTick`
  (params (DeltaSeconds :type "Float (single-precision)"))
  (bind _stickto (`self.stickTo`)
    (:`then`
      (`self.K2_SetActorLocation` (`SceneComponent.K2_GetComponentLocation` _stickto) true))
    (:`else`)))

(fn `setTarget`
  (params (newTarget :type "Actor Object Reference"))
  (bind _output_get (set `self.followTarget` newTarget))
  (`/Engine/EditorBlueprintResources/StandardMacros.IsValid` _output_get
    (:`Is Valid`
      (bind _interactiontransform (message `/Game/Blueprints/Interactive/BPI_Interactive.getInteractionTransform` (`self.followTarget`)))
      (`/Engine/EditorBlueprintResources/StandardMacros.IsValid` _interactiontransform
        (:`Is Valid`
          (set `self.stickTo` _interactiontransform))
        (:`Is Not Valid`
          (set `self.stickTo` (`Actor.RootComponent` (`self.followTarget`))))))
    (:`Is Not Valid`
      (set `self.stickTo` null))))

(fn `UserConstructionScript`)