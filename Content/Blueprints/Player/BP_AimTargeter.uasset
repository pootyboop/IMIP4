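; VR hand targeter for aim-assisted, rhythm-timed grabbing of electricity, liquids and other interactables.
; A capsule gathers overlaps, filters them by targeting mode and properties, and points a spawned BP_AimAssister at the one nearest their average location.
; Grab and drop resolve inside the beat's error margin, buffering early input; grabs can spawn electricity chainers or draw water.
; Each beat updates haptics and lerps the held object toward the assister's target.
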(event `self.ReceiveBeginPlay`
  (set `self.currMode` (`self.defaultMode`))
  (`self.updateInMenu`)
  (set `self.player` (cast `/Game/VRTemplate/Blueprints/VRPawn` (`self.GetAttachParentActor`) :!pure true))
  (bind _returnvalue (`|SpawnActorFromClass` "/Game/Blueprints/Player/BP_AimAssister.BP_AimAssister_C" (`self.GetTransform`) "Undefined" "MultiplyWithRoot" null self null))
  (set `self.aimAssister` _returnvalue)
  (`KismetSystemLibrary.K2_SetTimerDelegate` (delegate `BindBeatEvents`) (`/Game/Blueprints/BPFL_BlueprintFunctionLibrary.getBeatStartDelay` true)))

(event `BindBeatEvents`
  (`/Game/Blueprints/BPFL_BlueprintFunctionLibrary.bindEventToRhythm` "NewEnumerator1" (`|CreateDelegate` :!event `OnBeat`))
  (`/Game/Blueprints/BPFL_BlueprintFunctionLibrary.bindEventToRhythm` "NewEnumerator3" (`|CreateDelegate` :!event `ErrorMarginStarted`))
  (`/Game/Blueprints/BPFL_BlueprintFunctionLibrary.bindEventToRhythm` "NewEnumerator4" (`|CreateDelegate` :!event `ErrorMarginEnded`)))

(event `OnBeat`
  ;[1 1 1] Beat
  (`self.updateHaptics`)
  (`self.LerpGrabbedToPoint`))

(event `LerpGrabbedToPoint`
  ;[1 1 1] LERP Move
  (bind _grabbedobject (`self.grabbedObject`)
    (:`then`
      (set `self.grabbedPreLerpPos` (`self.K2_GetActorLocation` _grabbedobject))
      (bind (_direction _alpha) (`Timeline|MoveLERP` :!via `PlayFromStart` :!label _label)
        (:`Update`
          (`self.grabbedObject`
            (:`then`
              (`self.K2_SetActorLocation` (`self.grabbedObject`) (`KismetMathLibrary.VLerp` (`self.grabbedPreLerpPos`) (`self.K2_GetActorLocation` (`/Game/Blueprints/Player/BP_AimAssister.followTarget` (`self.aimAssister`))) _alpha) true false))
            (:`else`
              (goto _label :!via `Stop`))))))
    (:`else`)))

(event `self.AimAssistCapsule.OnComponentBeginOverlap`
  (params (OverlappedComponent :type "PrimitiveComponent Object Reference") (OtherActor :type "Actor Object Reference") (OtherComp :type "PrimitiveComponent Object Reference") (OtherBodyIndex :type Integer) (bFromSweep :type Boolean) (SweepResult :type "HitResult Structure (by ref)"))
  ;[1 1 1] Overlap
  (if (`/Game/VRTemplate/Blueprints/VRPawn.isAlive` (`self.player`))
    (`KismetArrayLibrary.Array_AddUnique` (`self.overlappedInteractables`) OtherActor)
    (`self.tryAddObject` OtherActor)))

(event `self.AimAssistCapsule.OnComponentEndOverlap`
  (params (OverlappedComponent :type "PrimitiveComponent Object Reference") (OtherActor :type "Actor Object Reference") (OtherComp :type "PrimitiveComponent Object Reference") (OtherBodyIndex :type Integer))
  ;[1 1 1] Overlap
  (if (`/Game/VRTemplate/Blueprints/VRPawn.isAlive` (`self.player`))
    (`KismetArrayLibrary.Array_RemoveItem` (`self.overlappedInteractables`) OtherActor)
    (`self.tryRemoveObject` OtherActor)))

(event `BeginInteraction`
  ;[1 1 1] On-time input
  (set `self.holdingInteract` true)
  (set `self.newActionAttempt` true)
  (if (`/Game/Blueprints/BPFL_BlueprintFunctionLibrary.isCurrentlyInErrorMargin`)
    (`self.grab`)))

(event `EndInteraction`
  ;[1 1 1] On-time input
  (set `self.holdingInteract` false)
  (set `self.newActionAttempt` true)
  (if (`/Game/Blueprints/BPFL_BlueprintFunctionLibrary.isCurrentlyInErrorMargin`)
    (`self.drop` false)))

(event `ErrorMarginStarted`
  ;[1 1 1] Auto input (Error Margin)
  (if (`self.newActionAttempt`)
    (if (`self.holdingInteract`)
      (`self.grab`)
      (else
        (`self.drop` false)))))

(event `ErrorMarginEnded`
  ;[1 1 1] Auto input (Error Margin)
  (set `self.newActionAttempt` false))

(event `OnGrabbedEndPlay`
  (params (Actor :type "Actor Object Reference") (EndPlayReason :type "EEndPlayReason Enum" :default "Destroyed"))
  (`self.drop` true))

(fn `drop`
  (params (forceDrop :type Boolean))
  (`|ExecutionSequence`
    (:`then_0`
      (bind _grabbedobject (`self.grabbedObject`)
        (:`then`
          (message `/Game/Blueprints/Interactive/BPI_Interactive.interactStop` _grabbedobject null "NewEnumerator5")
          (message `/Game/Blueprints/Interactive/BPI_Interactive.stopGrab` _grabbedobject)
          (set `self.grabbedObject` null :!label _label)
          (`self.updateHaptics`)
          (set `self.currMode` (`self.defaultMode`))
          (`self.refreshOverlappedTargetables`)
          (`/Game/VRTemplate/Blueprints/VRPawn.setHandGrabState` (cast `/Game/VRTemplate/Blueprints/VRPawn` (`self.GetOwner`) :!pure true) false (`self.isRight`) false))
        (:`else`
          (if (`local.forceDrop`)
            (goto _label)))))
    (:`then_1`
      (set `self.newActionAttempt` false))))

(fn `findAssistedTarget`
  (returns (newTarget :type "Actor Object Reference") (oldTarget :type "Actor Object Reference"))
  (locals (actorLoc :type "Vector Structure" :default (0.0 0.0 0.0)) (currDist :type "Float (double-precision)" :default 0.0) (nearestDist :type "Float (double-precision)" :default 10000000.0) (best :type "Actor Object Reference") (old :type "Actor Object Reference"))
  (set `local.old` (`/Game/Blueprints/Player/BP_AimAssister.followTarget` (`self.aimAssister`)))
  (set `local.best` self)
  (`|ExecutionSequence`
    (:`then_0`
      (bind _returnvalue (`GameplayStatics.GetActorArrayAverageLocation` (`self.overlappedTargetables`)))
      (set `local.actorLoc` _returnvalue)
      (for _array_element (`self.overlappedTargetables`)
        (bind _output_get (set `local.currDist` (`KismetMathLibrary.Vector_Distance` (`self.K2_GetActorLocation` _array_element) (`local.actorLoc`))))
        (if (< _output_get (`local.nearestDist`))
          (set `local.nearestDist` (`local.currDist`))
          (set `local.best` _array_element))))
    (:`then_1`
      (return (`local.best`) (`local.old`)))))

(fn `grab`
  (locals (props :type "Array of /Game/Blueprints/Interactive/EInteractiveProperty Enum"))
  (bind _props (`local.props`))
  (bind _grabbedobject (`self.grabbedObject`))
  (`self.drop` false)
  (bind _followtarget (`/Game/Blueprints/Player/BP_AimAssister.followTarget` (`self.aimAssister`))
    (:`then`
      (if (!= _followtarget self)
        (set `self.grabbedObject` _followtarget)
        (`self.updateHaptics`)
        (bind _properties (message `/Game/Blueprints/Interactive/BPI_Interactive.getProperties` (`self.grabbedObject`)))
        (set `local.props` _properties)
        (`|ExecutionSequence`
          (:`then_0`
            (if (`KismetArrayLibrary.Array_Contains` (`local.props`) "NewEnumerator14")
              (message `/Game/Blueprints/Interactive/BPI_Interactive.interactStart` (`self.grabbedObject`) null "NewEnumerator6")
              (return)))
          (:`then_1`
            ;[1 1 1] Regular grab
            (switch `/Game/Blueprints/Player/ETargeterMode` (`self.currMode`)
              (:`NewEnumerator1`
                (`|ExecutionSequence`
                  (:`then_0`
                    _)
                  (:`then_1`
                    (if (`KismetArrayLibrary.Array_Contains` (`local.props`) "NewEnumerator9") :!label _label
                      (`self.grabSuccessful` (`self.grabbedObject`) false true)
                      (return)
                      (else
                        (bind _liquidglob (message `/Game/Blueprints/Interactive/BPI_Interactive.drawWaterFrom` (`self.grabbedObject`)))
                        (`self.grabSuccessful` _liquidglob true true)
                        (`/Game/Blueprints/BPFL_BlueprintFunctionLibrary.tryPlayTrackByCondition` "NewEnumerator4")
                        (return))))))
              (:`NewEnumerator2`
                _)
              (:`NewEnumerator3`
                (set `self.currMode` "NewEnumerator0")
                (goto _label)))
            (set `self.currMode` "NewEnumerator0")
            (if (or (`KismetArrayLibrary.Array_Contains` _props "NewEnumerator7") (`KismetArrayLibrary.Array_Contains` _props "NewEnumerator6"))
              (bind _returnvalue (`|SpawnActorFromClass` "/Game/Blueprints/Player/Electricity/BP_ElectricityChainer.BP_ElectricityChainer_C" (`KismetMathLibrary.Conv_VectorToTransform` (`self.K2_GetActorLocation` _grabbedobject)) "Undefined" "MultiplyWithRoot" (`GameplayStatics.GetPlayerPawn` 0) _grabbedobject null))
              (`self.grabSuccessful` _returnvalue true)
              (`/Game/Blueprints/BPFL_BlueprintFunctionLibrary.tryPlayTrackByCondition` "NewEnumerator5")
              (return))))))
    (:`else`)))

(fn `grabSuccessful`
  (params (grabbedObject :type "Actor Object Reference") (freshSpawned :type Boolean) (isSecondaryColor :type Boolean))
  (set `self.grabbedObject` grabbedObject)
  (set `self.freshSpawned` freshSpawned)
  (message `/Game/Blueprints/Interactive/BPI_Interactive.startGrab` (`self.grabbedObject`) self)
  (message `/Game/Blueprints/Interactive/BPI_Interactive.setTargeted` (`self.grabbedObject`) false)
  (add `self.OnEndPlay` (`self.grabbedObject`) (`|CreateDelegate` :!event `OnGrabbedEndPlay`))
  (message `/Game/Blueprints/Interactive/BPI_Interactive.interactStart` (`self.grabbedObject`) null "NewEnumerator5")
  (`self.refreshOverlappedTargetables`)
  (`/Game/VRTemplate/Blueprints/VRPawn.setHandGrabState` (cast `/Game/VRTemplate/Blueprints/VRPawn` (`self.GetOwner`) :!pure true) true (`self.isRight`) (`local.isSecondaryColor`))
  (if (`/Game/Blueprints/BPFL_BlueprintFunctionLibrary.isCurrentlyInErrorMargin`)
    (`self.LerpGrabbedToPoint`)))

(fn `hasPropertiesForMode`
  (params (obj :type "Actor Object Reference"))
  (returns (result :type Boolean))
  (locals (props :type "Array of /Game/Blueprints/Interactive/EInteractiveProperty Enum"))
  (bind _props (`local.props`))
  (bind _props_2 (`local.props`))
  (bind _returnvalue (or (`KismetArrayLibrary.Array_Contains` _props "NewEnumerator6") (`KismetArrayLibrary.Array_Contains` _props "NewEnumerator7")))
  (bind _returnvalue_2 (or (`KismetArrayLibrary.Array_Contains` _props_2 "NewEnumerator2") (and (`KismetArrayLibrary.Array_Contains` _props_2 "NewEnumerator9") (not (`KismetArrayLibrary.Array_Contains` _props_2 "NewEnumerator10")))))
  (bind _properties (message `/Game/Blueprints/Interactive/BPI_Interactive.getProperties` obj))
  (bind _output_get (set `local.props` _properties))
  (if (`KismetArrayLibrary.Array_Contains` _output_get "NewEnumerator14")
    (return true)
    (else
      (switch `/Game/Blueprints/Player/ETargeterMode` (`self.currMode`)
        (:`NewEnumerator0`
          (return false))
        (:`NewEnumerator1`
          (`|ExecutionSequence`
            (:`then_0`
              _)
            (:`then_1`
              (return (or _returnvalue _returnvalue_2)))))
        (:`NewEnumerator2`
          (`|ExecutionSequence`
            (:`then_0`
              _)
            (:`then_1`
              (return _returnvalue))))
        (:`NewEnumerator3`
          (`|ExecutionSequence`
            (:`then_0`
              _)
            (:`then_1`
              (return _returnvalue_2)))))
      (if (not (`KismetArrayLibrary.Array_IsValidIndex` (`local.props`)))
        (return false)))))

(fn `refreshOverlappedTargetables`
  (`KismetArrayLibrary.Array_Clear` (`self.overlappedTargetables`))
  (for _array_element (`self.overlappedInteractables`)
    (`self.tryAddObject` _array_element false))
  (`self.updateAimTarget`))

(fn `tryAddObject`
  (params (obj :type "Actor Object Reference (by ref)") (updateAimTarget :type Boolean :default true))
  (if (and (`self.hasPropertiesForMode` obj) (`/Game/VRTemplate/Blueprints/VRPawn.isAlive` (`self.player`)))
    (`KismetArrayLibrary.Array_Add` (`self.overlappedTargetables`) (`local.obj`))
    (if (`local.updateAimTarget`)
      (`self.updateAimTarget`))))

(fn `tryRemoveObject`
  (params (obj :type "Actor Object Reference"))
  (`KismetArrayLibrary.Array_RemoveItem` (`self.overlappedTargetables`) obj)
  (`self.updateAimTarget`))

(fn `updateAimTarget`
  (bind (_newtarget _oldtarget) (`self.findAssistedTarget`))
  (message `/Game/Blueprints/Interactive/BPI_Interactive.setTargeted` _oldtarget false)
  (message `/Game/Blueprints/Interactive/BPI_Interactive.setTargeted` _newtarget true)
  (set `/Game/Blueprints/Player/BP_AimAssister.followTarget` _newtarget (`self.aimAssister`)))

(fn `updateCapsuleSize`
  (`CapsuleComponent.SetCapsuleHalfHeight` (`self.AimAssistCapsule`) (`self.aimAssistHalfHeight`) true)
  (`CapsuleComponent.SetCapsuleRadius` (`self.AimAssistCapsule`) (`self.aimAssistRadius`) true))

(fn `updateHaptics`
  (locals (newHapticsState :type Boolean))
  (bind _returnvalue (`GameplayStatics.GetPlayerController` 0))
  (bind _newhapticsstate (`local.newHapticsState`))
  (`|ExecutionSequence`
    (:`then_0`
      (set `local.newHapticsState` (`KismetSystemLibrary.IsValid` (`self.grabbedObject`)))
      (if (not (and (== (`self.hapticsState`) _newhapticsstate) (== _newhapticsstate false)))
        (`/Engine/EditorBlueprintResources/StandardMacros.IsValid` _returnvalue
          (:`Is Valid`
            (`PlayerController.SetHapticsByValue` _returnvalue 0.0 (`KismetMathLibrary.SelectFloat` (`self.grabHapticStrength`) 0.0 (`local.newHapticsState`)) (select `bool` (`self.isRight`) :`false` "Left" :`true` "Right" :!type "EControllerHand Enum"))))))
    (:`then_1`
      (set `self.hapticsState` (`local.newHapticsState`)))))

(fn `updateInMenu`
  (bind _output_get (set `self.isInMenu` (`/Game/Blueprints/BPFL_BlueprintFunctionLibrary.isInMenu`)))
  (set `self.aimAssistRadius` (`KismetMathLibrary.SelectFloat` 10.0 150.0 _output_get))
  (`SceneComponent.K2_SetRelativeLocation` (`self.Sphere`) (`KismetMathLibrary.MakeVector` (`KismetMathLibrary.SelectFloat` -300.0 0.0 (`self.isInMenu`))) false true)
  (`self.updateCapsuleSize`))

(fn `UserConstructionScript`
  (`self.updateCapsuleSize`)
  (`SceneComponent.SetHiddenInGame` (`self.AimAssistCapsule`) (not (`self.debugInfo`)) false))