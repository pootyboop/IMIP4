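; Grabbable-style electricity chainer that links actors with electricity chain segments and destroys itself when the grab stops.
; It starts a chain from StartChainedTo, then extends it to overlapped actors that answer the interact message with a valid electrified FX.
; Each link pins the current segment to the new actor and spawns another trailing to the chainer, tracked in a map.
; Destruction notifies chained actors and removes all segments and BP_Electrified start effects.
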(event `self.ReceiveBeginPlay`
  (`self.newChain` (`self.startChainedTo`)))

(event `self.ReceiveDestroyed`
  (`self.endElectricityChain`))

(event `self.Overlap.OnComponentBeginOverlap`
  (params (OverlappedComponent :type "PrimitiveComponent Object Reference") (OtherActor :type "Actor Object Reference") (OtherComp :type "PrimitiveComponent Object Reference") (OtherBodyIndex :type Integer) (bFromSweep :type Boolean) (SweepResult :type "HitResult Structure (by ref)"))
  (bind _electrifiedfx (message `/Game/Blueprints/Interactive/BPI_Interactive.interactStart` OtherActor null "NewEnumerator4"))
  (`/Engine/EditorBlueprintResources/StandardMacros.IsValid` _electrifiedfx
    (:`Is Valid`
      (`self.newChain` OtherActor _electrifiedfx))))

(event `self.Overlap.OnComponentEndOverlap`
  (params (OverlappedComponent :type "PrimitiveComponent Object Reference") (OtherActor :type "Actor Object Reference") (OtherComp :type "PrimitiveComponent Object Reference") (OtherBodyIndex :type Integer))
  (message `/Game/Blueprints/Interactive/BPI_Interactive.interactStop` OtherActor null "NewEnumerator4"))

(event `/Game/Blueprints/Interactive/BPI_Interactive.stopGrab`
  (`self.K2_DestroyActor`))

(fn `correctChainPoint`
  (params (actor :type "Actor Object Reference"))
  (returns (ReturnValue :type "Vector Structure"))
  (bind _interactiontransform (message `/Game/Blueprints/Interactive/BPI_Interactive.getInteractionTransform` actor))
  (`/Engine/EditorBlueprintResources/StandardMacros.IsValid` _interactiontransform
    (:`Is Valid`
      (return (`SceneComponent.K2_GetComponentLocation` _interactiontransform)))
    (:`Is Not Valid`
      (return (`self.K2_GetActorLocation` actor)))))

(fn `drawWaterFrom`
  (returns (liquidGlob :type "/Game/Blueprints/Player/LiquidGlob/BP_LiquidGlob Object Reference"))
  (return null))

(fn `endElectricityChain`
  (bind _keys (`BlueprintMapLibrary.Map_Keys` (`self.chain`)))
  (for _array_element _keys
    (message `/Game/Blueprints/Interactive/BPI_Interactive.endChain` (`BlueprintMapLibrary.Map_Find` (`self.chain`) _array_element))
    (bind _start (`/Game/Blueprints/Player/Electricity/BP_ElectricityChain.start` _array_element)
      (:`then`
        (if (== (`GameplayStatics.GetObjectClass` _start) "/Game/Blueprints/Player/Electricity/BP_Electrified.BP_Electrified_C")
          (`self.K2_DestroyActor` _start)))
      (:`else`
        _))
    (`self.K2_DestroyActor` _array_element)))

(fn `getCorrectStart`
  (params (electrifiedFX :type "/Game/Blueprints/Player/Electricity/BP_Electrified Object Reference") (actor :type "Actor Object Reference"))
  (returns (out :type "Actor Object Reference"))
  (`/Engine/EditorBlueprintResources/StandardMacros.IsValid` electrifiedFX
    (:`Is Valid`
      (return electrifiedFX))
    (:`Is Not Valid`
      (return actor))))

(fn `getGrabPhysicsSimulators`
  (returns (physicsSimulators :type "Array of PrimitiveComponent Object Reference"))
  (return))

(fn `getInteractionTransform`
  (returns (interactionTransform :type "SceneComponent Object Reference"))
  (return null))

(fn `getProperties`
  (returns (properties :type "Array of /Game/Blueprints/Interactive/EInteractiveProperty Enum"))
  (return))

(fn `interactStart`
  (params (caller :type "/Game/Blueprints/Interactive/BPI_Interactive Interface") (interactionType :type "/Game/Blueprints/Interactive/EInteractionType Enum" :default "NewEnumerator0"))
  (returns (electrifiedFX :type "/Game/Blueprints/Player/Electricity/BP_Electrified Object Reference") (isGrabbable :type Boolean))
  (return null false))

(fn `newChain`
  (params (chainedToActor :type "Actor Object Reference") (electrifiedFX :type "/Game/Blueprints/Player/Electricity/BP_Electrified Object Reference"))
  (`/Engine/EditorBlueprintResources/StandardMacros.IsValid` chainedToActor
    (:`Is Valid`
      (bind _currchain (`self.currChain`)
        (:`then`
          (`/Game/Blueprints/Player/Electricity/BP_ElectricityChain.setChainablePoints` _currchain (`/Game/Blueprints/Player/Electricity/BP_ElectricityChain.start` _currchain) (`local.chainedToActor`)))
        (:`else`
          _))
      (bind _returnvalue (`|SpawnActorFromClass` "/Game/Blueprints/Player/Electricity/BP_ElectricityChain.BP_ElectricityChain_C" (`KismetMathLibrary.Conv_VectorToTransform` (`self.correctChainPoint` (`local.chainedToActor`))) "Undefined" "MultiplyWithRoot" null (`self.getCorrectStart` (`local.electrifiedFX`) (`local.chainedToActor`)) self null))
      (bind _output_get (set `self.currChain` _returnvalue))
      (`BlueprintMapLibrary.Map_Add` (`self.chain`) _output_get (`local.chainedToActor`)))))

(fn `startElectrified`
  (returns (electrifiedFX :type "/Game/Blueprints/Player/Electricity/BP_Electrified Object Reference"))
  (return null))

(fn `UserConstructionScript`)