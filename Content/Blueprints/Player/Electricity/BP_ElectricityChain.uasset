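; Electricity chain effect actor that draws a particle link between a Start actor and an End actor.
; Construction tints the particles, then SetChainablePoints stores both actors and snaps the chain to Start's location by attachment, keeping world rotation.
; Every tick it feeds the unrotated world-space offset to End into the "ChainEnd" particle parameter, falling back to a fixed X offset when End is invalid.
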(event `self.ReceiveTick`
  (params (DeltaSeconds :type "Float (single-precision)"))
  (`self.updateChainEndLocation`))

(fn `setChainablePoints`
  (params (start :type "Actor Object Reference") (end :type "Actor Object Reference"))
  (`|ExecutionSequence`
    (:`then_0`
      (bind _output_get (set `self.start` start))
      (`self.K2_AttachToActor` _output_get "None" "SnapToTarget" "KeepWorld" "KeepWorld"))
    (:`then_1`
      (set `self.end` end)
      (`self.updateChainEndLocation`))))

(fn `updateChainEndLocation`
  (bind _end (`self.end`)
    (:`then`
      (`FXSystemComponent.SetVectorParameter` (`self.Particles`) "ChainEnd" (- (`self.K2_GetActorLocation` _end) (`SceneComponent.K2_GetComponentLocation` (`self.DefaultSceneRoot`)))))
    (:`else`
      (`FXSystemComponent.SetVectorParameter` (`self.Particles`) "ChainEnd" (200.0 0.0 0.0)) ; Default pos
    )))

(fn `UserConstructionScript`
  (`/Game/Blueprints/BPFL_BlueprintFunctionLibrary.setElectricityColor` (`self.Particles`))
  (`self.setChainablePoints` (`self.start`) (`self.end`)))