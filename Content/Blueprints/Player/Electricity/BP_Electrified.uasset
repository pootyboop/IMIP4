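; BP_Electrified is an electricity effect actor that can be attached to another component or actor.
; Its construction script colors two particle components, then attaches to AttachToComponent if valid, otherwise to AttachToActor.
; Attachment snaps location and scale to the target but keeps world rotation.
; BeginPlay reapplies the electricity colors at full intensity through the same shared function.
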(event `self.ReceiveBeginPlay`
  (`self.setElectricityColors`))

(fn `setElectricityColors`
  (`/Game/Blueprints/BPFL_BlueprintFunctionLibrary.setElectricityColor` (`self.Particles`))
  (`/Game/Blueprints/BPFL_BlueprintFunctionLibrary.setElectricityColor` (`self.Particles1`)))

(fn `UserConstructionScript`
  (`self.setElectricityColors`)
  (bind _attachtocomponent (`self.attachToComponent`)
    (:`then`
      (`self.K2_AttachToComponent` _attachtocomponent "None" "SnapToTarget" "KeepWorld" "SnapToTarget"))
    (:`else`
      (bind _attachtoactor (`self.attachToActor`)
        (:`then`
          (`self.K2_AttachToActor` _attachtoactor "None" "SnapToTarget" "KeepWorld" "SnapToTarget"))
        (:`else`)))))