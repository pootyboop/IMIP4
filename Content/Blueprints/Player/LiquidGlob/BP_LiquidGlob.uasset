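; BP_LiquidGlob is a controllable liquid glob that grabs interactable actors it overlaps.
; Each new grab spawns a BP_LiquidGrabbed proxy and attaches the actor to it, superseding a disconnected physics-constraint approach.
; DropGlob releases control and enables physics and collision on Block.
; A hit or StopGrab on an uncontrolled glob notifies proxies of the drop, then a timeline animates scale before destroying it.
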(event `self.ReceiveBeginPlay`
  (`PrimitiveComponent.SetCollisionEnabled` (`self.Block`) "NoCollision"))

(event `self.Overlap.OnComponentBeginOverlap`
  (params (OverlappedComponent :type "PrimitiveComponent Object Reference") (OtherActor :type "Actor Object Reference") (OtherComp :type "PrimitiveComponent Object Reference") (OtherBodyIndex :type Integer) (bFromSweep :type Boolean) (SweepResult :type "HitResult Structure (by ref)"))
  (bind (_electrifiedfx _isgrabbable) (message `/Game/Blueprints/Interactive/BPI_Interactive.interactStart` OtherActor null "NewEnumerator2"))
  (if _isgrabbable
    (bind _success (`self.tryGrabActor` OtherActor))
    (if _success
      (message `/Game/Blueprints/Interactive/BPI_Interactive.startGrab` OtherActor))))

(event `self.Overlap.OnComponentEndOverlap`
  (params (OverlappedComponent :type "PrimitiveComponent Object Reference") (OtherActor :type "Actor Object Reference") (OtherComp :type "PrimitiveComponent Object Reference") (OtherBodyIndex :type Integer))
  (message `/Game/Blueprints/Interactive/BPI_Interactive.interactStop` OtherActor null "NewEnumerator2")
  (message `/Game/Blueprints/Interactive/BPI_Interactive.stopGrab` OtherActor))

(event `self.ReceiveTick`
  (params (DeltaSeconds :type "Float (single-precision)")))

(event `self.ReceiveHit`
  (params (MyComp :type "PrimitiveComponent Object Reference") (Other :type "Actor Object Reference") (OtherComp :type "PrimitiveComponent Object Reference") (bSelfMoved :type Boolean) (HitLocation :type "Vector Structure") (HitNormal :type "Vector Structure") (NormalImpulse :type "Vector Structure") (Hit :type "HitResult Structure (by ref)"))
  (`self.TryDie`))

(event `TryDie`
  (if (`KismetMathLibrary.BooleanNOR` (`self.controlled`) (`self.grounded`))
    (`self.globHitGround`)))

(event `DeathTimeline`
  (bind (_direction _alpha) (`Timeline|Timeline` :!via `PlayFromStart`)
    (:`Update`
      (`self.SetActorScale3D` (`KismetMathLibrary.Conv_DoubleToVector` _alpha)))
    (:`Finished`
      (`self.K2_DestroyActor`))))

(event `/Game/Blueprints/Interactive/BPI_Interactive.stopGrab`
  (set `self.controlled` false)
  (`self.TryDie`))

(fn `drawWaterFrom`
  (returns (liquidGlob :type "/Game/Blueprints/Player/LiquidGlob/BP_LiquidGlob Object Reference"))
  (return null))

(fn `dropGlob`
  (if (`self.controlled`)
    (set `self.controlled` false)
    (`PrimitiveComponent.SetSimulatePhysics` (`self.Block`) true)
    (`PrimitiveComponent.SetCollisionEnabled` (`self.Block`) "QueryAndPhysics")))

(fn `getGrabPhysicsSimulators`
  (returns (physicsSimulators :type "Array of PrimitiveComponent Object Reference"))
  (return))

(fn `getProperties`
  (returns (properties :type "Array of /Game/Blueprints/Interactive/EInteractiveProperty Enum"))
  (return))

(fn `globHitGround`
  (set `self.grounded` true)
  (for _array_element (`self.liquidGrabs`)
    (`/Game/Blueprints/Player/LiquidGlob/BP_LiquidGrabbed.GlobDropped` _array_element))
  (`self.DeathTimeline`))

(fn `interactStart`
  (params (caller :type "/Game/Blueprints/Interactive/BPI_Interactive Interface") (interactionType :type "/Game/Blueprints/Interactive/EInteractionType Enum" :default "NewEnumerator0"))
  (returns (electrifiedFX :type "/Game/Blueprints/Player/Electricity/BP_Electrified Object Reference") (isGrabbable :type Boolean))
  (return null false))

(fn `startElectrified`
  (returns (electrifiedFX :type "/Game/Blueprints/Player/Electricity/BP_Electrified Object Reference"))
  (return null))

(fn `tryGrabActor`
  (params (grabbedActor :type "Actor Object Reference"))
  (returns (success :type Boolean))
  (locals (newPhysicsConstraint :type "PhysicsConstraintComponent Object Reference") (physicsComponent :type "PrimitiveComponent Object Reference") (liquidGrabbed :type "/Game/Blueprints/Player/LiquidGlob/BP_LiquidGrabbed Object Reference"))
  (bind _grabbedactor (`local.grabbedActor`))
  (bind (_returnvalue_location _returnvalue_rotation) (`KismetMathLibrary.BreakTransform` (`self.GetTransform` _grabbedactor)))
  (bind _values (`BlueprintMapLibrary.Map_Values` (`self.constraintMap`)))
  (if (not (`KismetArrayLibrary.Array_Contains` _values (`local.grabbedActor`)))
    (`|ExecutionSequence`
      (:`then_0`
        (bind _returnvalue (`|SpawnActorFromClass` "/Game/Blueprints/Player/LiquidGlob/BP_LiquidGrabbed.BP_LiquidGrabbed_C" (`KismetMathLibrary.MakeTransform` _returnvalue_location _returnvalue_rotation) "Undefined" "MultiplyWithRoot" null self _grabbedactor null))
        (bind _output_get (set `local.liquidGrabbed` _returnvalue))
        (`KismetArrayLibrary.Array_Add` (`self.liquidGrabs`) _output_get)
        (`self.K2_AttachToActor` (`local.grabbedActor`) (`local.liquidGrabbed`) "None" "KeepWorld" "KeepWorld" "KeepWorld" true)
        (return true)))
    (else
      (return false))))

(fn `UserConstructionScript`)