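; BP_LiquidGrabbed is a helper actor that pulls its Parent actor toward a LiquidGlob, as though caught in the liquid.
; Each tick until dropped, it moves Parent toward the glob at a distance-scaled speed, without sweeping, and tumbles it by random rotation rates.
; GlobDropped stops the pull, plays a timeline easing Parent's rotation back to zero, then destroys this helper actor.
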(event `self.ReceiveTick`
  (params (DeltaSeconds :type "Float (single-precision)"))
  (if (not (`self.dropped`))
    (`self.MoveToGlob`)))

(event `MoveToGlob`
  (bind _returnvalue (`GameplayStatics.GetWorldDeltaSeconds`))
  (bind _returnvalue_2 (`self.K2_GetActorLocation` (`self.parent`)))
  (bind _returnvalue_3 (`KismetMathLibrary.RandomFloatInRange` (`self.rotateSpeedMin`) (`self.rotateSpeedMax`)))
  (bind _returnvalue_4 (`self.K2_GetActorLocation` (`self.liquidGlob`)))
  (`self.K2_AddActorWorldOffset` (`self.parent`) (* (`KismetMathLibrary.Normal` (`KismetMathLibrary.Conv_RotatorToVector` (`KismetMathLibrary.FindLookAtRotation` _returnvalue_2 _returnvalue_4))) _returnvalue (`KismetMathLibrary.Vector_Distance` _returnvalue_2 _returnvalue_4) (`self.moveToLiquidSpeed`)) false false)
  (`self.K2_AddActorWorldRotation` (`self.parent`) (* (`KismetMathLibrary.MakeRotator` _returnvalue_3 _returnvalue_3 _returnvalue_3) _returnvalue) false false))

(event `GlobDropped`
  (set `self.dropped` true)
  (bind (_direction _alpha) (`Timeline|Timeline` :!via `PlayFromStart`)
    (:`Update`
      (`self.K2_SetActorRotation` (`self.parent`) (`KismetMathLibrary.RLerp` (`self.K2_GetActorRotation` (`self.parent`)) (struct) _alpha) false))
    (:`Finished`
      (`self.K2_DestroyActor`))))

(fn `UserConstructionScript`)