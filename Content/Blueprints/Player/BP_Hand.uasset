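; Player hand Blueprint that shows grab feedback through animation, glow, LED color and spin.
; BeginPlay caches the mesh's relative transform and creates dynamic materials for the LED slot and HandGlow mesh.
; SetGrabbing passes the state to AnimBP_Hand, toggles glow visibility, and sets material parameters for beat colors and primary or secondary color.
; While grabbing, a looping timer rotates the skeletal mesh in steps; releasing clears it without restoring rotation.
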(event `self.ReceiveBeginPlay`
  (set `self.ogTransform` (`SceneComponent.GetRelativeTransform` (`self.SkeletalMesh`)))
  (bind _returnvalue (`PrimitiveComponent.CreateDynamicMaterialInstance` (`self.SkeletalMesh`) 2 "/Game/Materials/LED/MI_LED_Primary.MI_LED_Primary" "None"))
  (bind _output_get (set `self.mat` _returnvalue))
  (`MaterialInstanceDynamic.SetScalarParameterValue` _output_get "UseBeatColors" 0.0)
  (bind _returnvalue_2 (`PrimitiveComponent.CreateDynamicMaterialInstance` (`self.HandGlow`) 0 "/Game/Materials/FXandParticles/M_HandGlow.M_HandGlow" "None"))
  (set `self.glow` _returnvalue_2))

(event `StartSpin`
  (`self.StopSpin`)
  (bind _returnvalue (`KismetSystemLibrary.K2_SetTimerDelegate` (delegate `Spin`) 0.1 true))
  (set `self.timerHandle` _returnvalue))

(event `Spin`
  (`SceneComponent.K2_AddLocalRotation` (`self.SkeletalMesh`) (`KismetMathLibrary.MakeRotator` 0.0 (`self.spinSpeed`)) false false))

(event `StopSpin`
  (`KismetSystemLibrary.K2_ClearAndInvalidateTimerHandle` (`self.timerHandle`)))

(fn `setGrabbing`
  (params (newGrabbing :type Boolean) (isSecondaryColor :type Boolean))
  (set `self.grabbing` newGrabbing)
  (`|ExecutionSequence`
    (:`then_0`
      (bind _asanim_bp_hand (cast `/Game/Meshes/Player/AnimBP_Hand` (`SkeletalMeshComponent.GetAnimInstance` (`self.SkeletalMesh`))))
      (set `/Game/Meshes/Player/AnimBP_Hand.isGrabbing` (`self.grabbing`) _asanim_bp_hand))
    (:`then_1`
      (`SceneComponent.SetVisibility` (`self.HandGlow`) (`self.grabbing`) false)
      (if (`self.grabbing`)
        (`MaterialInstanceDynamic.SetScalarParameterValue` (`self.glow`) "UseSecondary" (`KismetMathLibrary.SelectFloat` 1.0 0.0 (`local.isSecondaryColor`)))))
    (:`then_2`
      (if (`self.grabbing`)
        (`self.StartSpin`)
        (`MaterialInstanceDynamic.SetScalarParameterValue` (`self.mat`) "UseBeatColors" (`KismetMathLibrary.SelectFloat` 1.0 0.5 (`local.isSecondaryColor`)))
        (else
          (`self.StopSpin`)
          (`MaterialInstanceDynamic.SetScalarParameterValue` (`self.mat`) "UseBeatColors" 0.0))))))

(fn `UserConstructionScript`)