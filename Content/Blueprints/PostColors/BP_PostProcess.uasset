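; BP_PostProcess is a post-process actor that follows a saved setting and pulses with the beat.
; UpdateSettings, also run at BeginPlay, toggles its PostProcess component from the "Post Processing" setting and mirrors that state into the PostEnabled parameter of MPC_Colors.
; OnBeatIntensityFadeUpdate uses the beat fade value to interpolate two intensity settings upward and the vignette downward.
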(event `self.ReceiveBeginPlay`
  (`self.UpdateSettings`))

(event `UpdateSettings`
  (bind _output_get (set `PostProcessComponent.bEnabled` (== (`/Game/Blueprints/BPFL_BlueprintFunctionLibrary.getSavedSetting` "Post Processing") 1) (`self.PostProcess`)))
  (`KismetMaterialLibrary.SetScalarParameterValue` "/Game/Materials/_MPC/MPC_Colors.MPC_Colors" "PostEnabled" (`KismetMathLibrary.Conv_BoolToDouble` _output_get)))

(event `/Game/Blueprints/Music/BeatSync/BPI_BeatSync.OnBeatIntensityFadeUpdate`
  (params (BeatIntensityFade :type "Float (double-precision)") (`Off-beat` :type Boolean))
  (setmembers `PostProcessSettings` :`StructRef` (`PostProcessComponent.Settings` (`self.PostProcess`)) :`SceneFringeIntensity` (`KismetMathLibrary.Lerp` 0.15 0.84 BeatIntensityFade) :`BloomIntensity` (`KismetMathLibrary.Lerp` 8.0 10.0 BeatIntensityFade) :`VignetteIntensity` (`KismetMathLibrary.Lerp` 0.3 0.1 BeatIntensityFade)))

(fn `UserConstructionScript`)