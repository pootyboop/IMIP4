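; Interactive actor that shows one saved game setting and cycles through its named options when directly selected.
; Selection increments the value, wrapping to the first, then saves it with an update sent and bumps the refreshed text.
; A child BP_TitleBodyText actor displays the setting ID and current option name.
; PC-exclusive settings on Android display as unavailable and have a property removed from BPCInteractive at BeginPlay.
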(event `self.ReceiveBeginPlay`
  (`parent.ReceiveBeginPlay`)
  (`self.updateAppearance`)
  (`|ExecutionSequence`
    (:`then_0`
      (set `self.titleBodyRef` (cast `/Game/UI/BP_TitleBodyText` (`ChildActorComponent.ChildActor` (`self.TitleBodyText`)) :!pure true)))
    (:`then_1`
      (if (`self.isUnavailableForPlatform`)
        (`/Game/Blueprints/Interactive/BPC_Interactive.removeProperty` (`self.BPC_Interactive`) "NewEnumerator14")))))

(event `self.OnDirectSelected`
  (bind _returnvalue (+ (`/Game/Blueprints/BPFL_BlueprintFunctionLibrary.getSavedSetting` (`self.settingID`)) 1))
  (`parent.OnDirectSelected`)
  (`self.setNewSettingValue` (`KismetMathLibrary.SelectInt` 0 _returnvalue (> _returnvalue (- (`KismetArrayLibrary.Array_Length` (`self.settingNames`)) 1)))))

(fn `isUnavailableForPlatform`
  (returns (ReturnValue :type Boolean))
  (return (and (`KismetStringLibrary.EqualEqual_StrStr` (`GameplayStatics.GetPlatformName`) "Android") (`self.isPCExclusive`))))

(fn `setNewSettingValue`
  (params (value :type Integer) (sendUpdate :type Boolean :default true))
  (`/Game/Blueprints/BPFL_BlueprintFunctionLibrary.setSavedSetting` (`self.settingID`) value sendUpdate)
  (`self.updateTextAppearance`)
  (`/Game/UI/BP_TitleBodyText.bumpBodyText` (`self.titleBodyRef`)))

(fn `updateAppearance`
  (`self.updateTextAppearance`)
  (`StaticMeshComponent.SetStaticMesh` (`self.StaticMesh`) (`self.mesh_0`)))

(fn `updateTextAppearance`
  (`/Game/UI/BP_TitleBodyText.setText` (cast `/Game/UI/BP_TitleBodyText` (`ChildActorComponent.ChildActor` (`self.TitleBodyText`)) :!pure true) (`KismetTextLibrary.Conv_NameToText` (`self.settingID`)) (select `bool` (`self.isUnavailableForPlatform`) :`false` (`|GetArrayItem` (`self.settingNames`) (`/Game/Blueprints/BPFL_BlueprintFunctionLibrary.getSavedSetting` (`self.settingID`))) :`true` "Unavailable (PC Exclusive)")))

(fn `UserConstructionScript`
  (`parent.UserConstructionScript`)
  (`self.setMeshes` (`|MakeArray` (`self.StaticMesh`) :!type "MeshComponent Object Reference"))
  (`self.updateAppearance`))