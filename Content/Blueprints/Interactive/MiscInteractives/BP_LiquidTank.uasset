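; BP_LiquidTank is an interactive liquid tank that electrocutes and is then removed from the level when damaged or killed.
; Both damage and kill events share one path that calls Electrocute and then DestroyActor.
; A disconnected branch that would remove the tank from every BP_AimTargeter before destruction never runs.
; The construction script runs the parent's setup, then registers Mesh0 through SetMeshes.
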(event `self.OnDamaged`
  (`/Game/Blueprints/Interactive/BPI_Interactive.electrocute` :!label _label)
  (`self.K2_DestroyActor`))

(event `self.OnDestroyedKilled`
  (goto _label))

(fn `UserConstructionScript`
  (`parent.UserConstructionScript`)
  (`self.setMeshes` (`|MakeArray` (`self.Mesh_0`) :!type "MeshComponent Object Reference")))