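; BP_AreaClearArrow is an interactive arrow with body text, named as an area-clear indicator, that responds to wave enable and disable events.
; Both events call the parent implementation, then show or hide the BodyText component without propagating to its children.
; The construction script runs the parent's, then passes the Arrow component to SetMeshes.
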(event `self.Wave Enable`
  (`parent.Wave Enable`)
  (`SceneComponent.SetVisibility` (`self.BodyText`) true false))

(event `self.Wave Disable`
  (`parent.Wave Disable`)
  (`SceneComponent.SetVisibility` (`self.BodyText`) false false))

(fn `UserConstructionScript`
  (`parent.UserConstructionScript`)
  (`self.setMeshes` (`|MakeArray` (`self.Arrow`) :!type "MeshComponent Object Reference")))