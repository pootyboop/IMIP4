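; BP_Electrocution is a short-lived electrocution hazard that instakills what it touches and lasts for a set number of rhythm beats.
; On spawn it triggers a conditional track, then sends damage messages to destroyables within its scaled collision sphere, releasing any grabbed liquid globs or electricity chainers among them.
; Later overlaps receive the same damage message, filtered by its Destroys setting.
; A bound rhythm event counts beats and destroys the actor when BeatsToLast is reached.
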(event `self.ReceiveBeginPlay`
  (bind _returnvalue_x (`KismetMathLibrary.BreakVector` (`self.GetActorScale3D`)))
  (bind _collision (`self.Collision`))
  (`/Game/Blueprints/BPFL_BlueprintFunctionLibrary.bindEventToRhythm` "NewEnumerator1" (delegate `OnBeat`))
  (`/Game/Blueprints/BPFL_BlueprintFunctionLibrary.tryPlayTrackByCondition` "NewEnumerator1")
  (bind (_outactors _returnvalue) (`KismetSystemLibrary.SphereOverlapActors` (`SceneComponent.K2_GetComponentLocation` _collision) (* (`SphereComponent.SphereRadius` _collision) _returnvalue_x) (`|MakeArray` "ObjectTypeQuery1" "ObjectTypeQuery2" "ObjectTypeQuery3" "ObjectTypeQuery4" :!type "EObjectTypeQuery Enum") "/Game/Blueprints/Interactive/Destroyable/BPI_Destroyable.BPI_Destroyable_C"))
  (if _returnvalue
    (for _array_element _outactors
      (message `/Game/Blueprints/Interactive/Destroyable/BPI_Destroyable.Damage` _array_element 0 true (`self.destroys`))
      ;[1 1 1] Kill controlled elements when they're involved in an electrocution
      (bind _asbp_liquid_glob (cast `/Game/Blueprints/Player/LiquidGlob/BP_LiquidGlob` _array_element)
        (:`then`
          (message `/Game/Blueprints/Interactive/BPI_Interactive.stopGrab` _asbp_liquid_glob))
        (:`CastFailed`
          (bind _asbp_electricity_chainer (cast `/Game/Blueprints/Player/Electricity/BP_ElectricityChainer` _array_element))
          (message `/Game/Blueprints/Interactive/BPI_Interactive.stopGrab` _asbp_electricity_chainer))))))

(event `OnBeat`
  (bind _result (`/Engine/EditorBlueprintResources/StandardMacros.IncrementInt` (`self.currBeat`))
    (:`  `
      (if (== _result (`self.beatsToLast`))
        (`self.K2_DestroyActor`)))))

(event `self.Collision.OnComponentBeginOverlap`
  (params (OverlappedComponent :type "PrimitiveComponent Object Reference") (OtherActor :type "Actor Object Reference") (OtherComp :type "PrimitiveComponent Object Reference") (OtherBodyIndex :type Integer) (bFromSweep :type Boolean) (SweepResult :type "HitResult Structure (by ref)"))
  (message `/Game/Blueprints/Interactive/Destroyable/BPI_Destroyable.Damage` OtherActor 0 true (`self.destroys`)))

(fn `UserConstructionScript`)