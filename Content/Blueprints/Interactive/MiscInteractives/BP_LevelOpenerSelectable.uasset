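; A selectable interactive actor that opens a referenced level when it is directly selected.
; It extends a parent interactive class, calling the parent logic before adding the level load on selection.
; Construction registers its static mesh with the parent's mesh setup.
; A shared appearance update, run on construction and BeginPlay, applies the mesh and pushes interaction title and body to a BP_TitleBodyText child actor.
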(event `self.ReceiveBeginPlay`
  (`parent.ReceiveBeginPlay`)
  (`self.updateAppearance`))

(event `self.OnDirectSelected`
  (`parent.OnDirectSelected`)
  (`GameplayStatics.OpenLevelBySoftObjectPtr` (`self.level`)))

(fn `updateAppearance`
  (`/Game/UI/BP_TitleBodyText.setText` (cast `/Game/UI/BP_TitleBodyText` (`ChildActorComponent.ChildActor` (`self.ChildActor`)) :!pure true) (`self.interactionTitle`) (`self.interactionBody`))
  (`StaticMeshComponent.SetStaticMesh` (`self.StaticMesh`) (`self.mesh_0`)))

(fn `UserConstructionScript`
  (`parent.UserConstructionScript`)
  (`self.setMeshes` (`|MakeArray` (`self.StaticMesh`) :!type "MeshComponent Object Reference"))
  (`self.updateAppearance`))