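; Interactive component that lets its owner react to electricity, chaining, liquid, grabbing and smashing.
; An enum property list acts as both capabilities and current state, queried through branching HasProperty macros.
; InteractStart registers the caller, updates properties, sends owner messages for electrify, wet, electrocute or smash, and returns electrified FX and grabbability.
; InteractStop and EndChain clear temporary states, keeping electrification on sources, and on chained objects during InteractStop.
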(event `self.ReceiveBeginPlay`
  (`self.hasPropertyM` "NewEnumerator6"
    (:`true`
      (message `/Game/Blueprints/Interactive/BPI_Interactive.startElectrified` (`self.GetOwner`)))))

(event `/Game/Blueprints/Interactive/BPI_Interactive.interactStop`
  (params (caller :type "/Game/Blueprints/Interactive/BPI_Interactive Interface") (interactionType :type "/Game/Blueprints/Interactive/EInteractionType Enum" :default "NewEnumerator0"))
  (`self.registerCallerInteractive` caller false)
  (switch `/Game/Blueprints/Interactive/EInteractionType` interactionType
    (:`NewEnumerator1`
      (`self.hasPropertyM` "NewEnumerator7" :!label _label
        (:`true`
          (`self.hasPropertiesM` (`|MakeArray` "NewEnumerator8" "NewEnumerator6" :!type "/Game/Blueprints/Interactive/EInteractiveProperty Enum") true ; Only remove ELECTRIFIED if not chainable or a source
            (:`false`
              (`self.removeProperty` "NewEnumerator7")
              (message `/Game/Blueprints/Interactive/BPI_Interactive.stopElectrified` (`self.GetOwner`)))))))
    (:`NewEnumerator4`
      (goto _label))
    (:`NewEnumerator5`
      ;[1 1 1] Throw
      (`self.removeProperty` "NewEnumerator10"))))

(event `/Game/Blueprints/Interactive/BPI_Interactive.endChain`
  (`self.removeProperty` "NewEnumerator8")
  (`self.hasPropertyM` "NewEnumerator6"
    (:`false`
      (`self.removeProperty` "NewEnumerator7")
      (message `/Game/Blueprints/Interactive/BPI_Interactive.stopElectrified` (`self.GetOwner`)))))

(fn `addProperty`
  (params (newProperty :type "/Game/Blueprints/Interactive/EInteractiveProperty Enum" :default "NewEnumerator0"))
  (`KismetArrayLibrary.Array_AddUnique` (`self.interactiveProperties`) newProperty)
  (if (`self.printDebug`)
    (`KismetSystemLibrary.PrintString` (`KismetStringLibrary.Concat_StrStr` (`KismetSystemLibrary.GetDisplayName` self) " gains property " (`|GetEnumeratorNameAsString` newProperty)) true true (struct :`R` 1.0 :`G` 0.56948 :`B` 0.674055 :`A` 1.0))))

(fn `drawWaterFrom`
  (returns (liquidGlob :type "/Game/Blueprints/Player/LiquidGlob/BP_LiquidGlob Object Reference"))
  (return null))

(fn `getGrabPhysicsSimulators`
  (returns (physicsSimulators :type "Array of PrimitiveComponent Object Reference"))
  (return))

(fn `getInteractionTransform`
  (returns (interactionTransform :type "SceneComponent Object Reference"))
  (return null))

(fn `getProperties`
  (returns (properties :type "Array of /Game/Blueprints/Interactive/EInteractiveProperty Enum"))
  (return (`self.interactiveProperties`)))

(fn `hasProperties`
  (params (properties :type "Array of /Game/Blueprints/Interactive/EInteractiveProperty Enum") (anyNotAll :type Boolean))
  (returns (ReturnValue :type Boolean))
  (for _array_element properties
    (if (`KismetArrayLibrary.Array_Contains` (`self.interactiveProperties`) _array_element)
      ;[1 1 1] Any was found
      (if (`local.anyNotAll`)
        (return true))
      (else
        ;[1 1 1] Not all was found
        (if (not (`local.anyNotAll`))
          (return false)))))
  ;[1 1 1] All was found OR any was not found
  (return (not (`local.anyNotAll`))))

(fn `hasProperty`
  (params (property :type "/Game/Blueprints/Interactive/EInteractiveProperty Enum" :default "NewEnumerator0"))
  (returns (ReturnValue :type Boolean))
  (return (`KismetArrayLibrary.Array_Contains` (`self.interactiveProperties`) property)))

(fn `interactStart`
  (params (caller :type "/Game/Blueprints/Interactive/BPI_Interactive Interface") (interactionType :type "/Game/Blueprints/Interactive/EInteractionType Enum" :default "NewEnumerator0"))
  (returns (electrifiedFX :type "/Game/Blueprints/Player/Electricity/BP_Electrified Object Reference") (isGrabbable :type Boolean))
  (set `self.electrifiedFX` null) ; Couldn't write to this as local :(
  (`|ExecutionSequence`
    (:`then_0`
      (`self.registerCallerInteractive` caller)
      (switch `/Game/Blueprints/Interactive/EInteractionType` interactionType
        (:`NewEnumerator1`
          (`|ExecutionSequence`
            (:`then_0`
              ;[1 1 1] Electrify
              (`self.hasPropertyM` "NewEnumerator7" :!label _label
                (:`false`
                  (`self.addProperty` "NewEnumerator7")
                  (bind _electrifiedfx (message `/Game/Blueprints/Interactive/BPI_Interactive.startElectrified` (`self.GetOwner`)))
                  (set `self.electrifiedFX` _electrifiedfx))))
            (:`then_1`
              ;[1 1 1] Electrocute
              (`self.hasPropertiesM` (`|MakeArray` "NewEnumerator1" "NewEnumerator2" :!type "/Game/Blueprints/Interactive/EInteractiveProperty Enum") true :!label _label_2
                (:`true`
                  (message `/Game/Blueprints/Interactive/BPI_Interactive.electrocute` (`self.GetOwner`)))))))
        (:`NewEnumerator4`
          (`|ExecutionSequence`
            (:`then_0`
              (goto _label))
            (:`then_1`
              ;[1 1 1] Chain
              (`self.hasPropertiesM` (`|MakeArray` "NewEnumerator3" "NewEnumerator6" :!type "/Game/Blueprints/Interactive/EInteractiveProperty Enum") true
                (:`true`
                  (`self.addProperty` "NewEnumerator8"))
                (:`false`
                  (set `self.electrifiedFX` null) ; Set to null so this isn't chained
                )))
            (:`then_2`
              (goto _label_2))))
        (:`NewEnumerator2`
          (`|ExecutionSequence`
            (:`then_0`
              ;[1 1 1] Wet
              (`self.hasPropertyM` "NewEnumerator4"
                (:`true`
                  (`self.hasPropertyM` "NewEnumerator1"
                    (:`false`
                      (`self.addProperty` "NewEnumerator1")
                      (message `/Game/Blueprints/Interactive/BPI_Interactive.startWet` (`self.GetOwner`)))))))
            (:`then_1`
              ;[1 1 1] Electrocute
              (`self.hasPropertiesM` (`|MakeArray` "NewEnumerator7" "NewEnumerator6" :!type "/Game/Blueprints/Interactive/EInteractiveProperty Enum") true
                (:`true`
                  (message `/Game/Blueprints/Interactive/BPI_Interactive.electrocute` (`self.GetOwner`)))))))
        (:`NewEnumerator5`
          (`self.hasPropertyM` "NewEnumerator9"
            (:`true`
              (`self.addProperty` "NewEnumerator10"))))
        (:`NewEnumerator3`
          ;[1 1 1] Smash
          (`self.hasPropertyM` "NewEnumerator5"
            (:`true`
              (message `/Game/Blueprints/Interactive/BPI_Interactive.smash` (`self.GetOwner`)))))))
    (:`then_1`
      (return (`self.electrifiedFX`) (and (`self.hasProperty` "NewEnumerator9") (not (`self.hasProperty` "NewEnumerator10")))))))

(fn `registerCallerInteractive`
  (params (callerInteractive :type "/Game/Blueprints/Interactive/BPI_Interactive Interface") (register :type Boolean :default true))
  (bind _callerinteractives (`self.callerInteractives`))
  (if register
    (`KismetArrayLibrary.Array_AddUnique` _callerinteractives callerInteractive)
    (else
      (`KismetArrayLibrary.Array_RemoveItem` _callerinteractives callerInteractive))))

(fn `removeProperty`
  (params (newProperty :type "/Game/Blueprints/Interactive/EInteractiveProperty Enum" :default "NewEnumerator0"))
  (`KismetArrayLibrary.Array_RemoveItem` (`self.interactiveProperties`) newProperty))

(fn `setPropertyHeld`
  (params (property :type "/Game/Blueprints/Interactive/EInteractiveProperty Enum" :default "NewEnumerator0") (newHeldState :type Boolean))
  (if newHeldState
    (`self.addProperty` property)
    (else
      (`self.removeProperty` property))))

(fn `startElectrified`)