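; Base actor for interactive objects that can be grabbed, highlighted, wetted, electrified, damaged and destroyed.
; It delegates grab, chain and most interaction logic to BPCInteractive, whose throw update is bound to the rhythm system.
; Targeting shows lazily created, collision-free duplicate meshes with outline materials, while wetness drives dynamic material parameters.
; Property- and type-gated damage feeds overridable hooks, and wave interactions toggle mesh visibility and actor collision.
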(event `self.ReceiveBeginPlay`
  (add `self.OnDestroyed` (delegate `OnDestroyed_Event`))
  (`KismetSystemLibrary.K2_SetTimerDelegate` (delegate `BeatBinding_Grabbed`) (`/Game/Blueprints/BPFL_BlueprintFunctionLibrary.getBeatStartDelay` true)))

(event `OnDestroyed_Event` :!signature `self.OnDestroyed`
  (params (DestroyedActor :type "Actor Object Reference"))
  (`/Game/Blueprints/Interactive/BPI_Interactive.stopElectrified`))

(event `BeatBinding_Grabbed`
  (`/Game/Blueprints/BPFL_BlueprintFunctionLibrary.bindEventToRhythm` "NewEnumerator4" (delegate `OnErrorMarginEnd_Grabbed`)))

(event `OnErrorMarginEnd_Grabbed`
  (`/Game/Blueprints/Interactive/BPC_Interactive.updateThrow` (`self.BPC_Interactive`)))

(event `/Game/Blueprints/Interactive/BPI_Interactive.stopElectrified`
  ;[1 1 1] Pass collision-based interface events to component
  (bind _electrifiedfx (`self.electrifiedFX`)
    (:`then`
      (`self.K2_DestroyActor` _electrifiedfx))
    (:`else`)))

(event `/Game/Blueprints/Interactive/BPI_Interactive.endChain`
  ;[1 1 1] Pass collision-based interface events to component
  (`/Game/Blueprints/Interactive/BPI_Interactive.endChain` (`self.BPC_Interactive`)))

(event `/Game/Blueprints/Interactive/BPI_Interactive.startGrab`
  (params (grabber :type "/Game/Blueprints/Player/BP_AimTargeter Object Reference"))
  (bind _bpc_interactive (`self.BPC_Interactive`))
  (if (`/Game/Blueprints/Interactive/BPC_Interactive.hasProperty` (`self.BPC_Interactive`) "NewEnumerator9")
    (`/Game/Blueprints/Interactive/BPC_Interactive.addProperty` _bpc_interactive "NewEnumerator10")
    (set `/Game/Blueprints/Interactive/BPC_Interactive.grabber` grabber _bpc_interactive)))

(event `/Game/Blueprints/Interactive/BPI_Interactive.stopGrab`
  (bind _bpc_interactive (`self.BPC_Interactive`))
  (`/Game/Blueprints/Interactive/BPC_Interactive.removeProperty` _bpc_interactive "NewEnumerator10")
  (set `/Game/Blueprints/Interactive/BPC_Interactive.grabber` null _bpc_interactive))

(event `/Game/Blueprints/Interactive/BPI_Interactive.setTargeted`
  (params (newTargeted :type Boolean))
  (`self.setHighlighted` newTargeted))

(event `/Game/Blueprints/Interactive/BPI_Interactive.startWet`
  (`self.setMaterialScalar` "Wetness" 1.0))

(event `/Game/Blueprints/Interactive/Destroyable/BPI_Destroyable.Damage`
  (params (damage :type Integer) (instakill :type Boolean) (canDamage :type "/Game/Blueprints/Interactive/Destroyable/EDestroyableType Enum" :default "NewEnumerator4"))
  ;[1 1 1] DamageDeath
  (if (and (`/Game/Blueprints/Interactive/BPC_Interactive.hasProperty` (`self.BPC_Interactive`) "NewEnumerator11") (or (`|EnumEquality` canDamage (`self.destroyableType`)) (`|EnumEquality` canDamage "NewEnumerator5") (and (`|EnumEquality` canDamage "NewEnumerator4") (or (`|EnumEquality` (`self.destroyableType`) "NewEnumerator1") (`|EnumEquality` (`self.destroyableType`) "NewEnumerator3")))))
    (if instakill
      (set `self.health` 0)
      (`self.OnDestroyedKilled` :!label _label)
      (else
        (bind _output_get (set `self.health` (- (`self.health`) damage)))
        (`self.OnDamaged`)
        (if (<= _output_get 0)
          (goto _label))))))

(event `OnDamaged`
  ;[1 1 1] DamageDeath
)

(event `OnDestroyedKilled`
  ;[1 1 1] DamageDeath
)

(event `/Game/Blueprints/Interactive/BPI_Interactive.electrocute`
  (`|SpawnActorFromClass` "/Game/Blueprints/Interactive/MiscInteractives/BP_Electrocution.BP_Electrocution_C" (`KismetMathLibrary.Conv_VectorToTransform` (`SceneComponent.K2_GetComponentLocation` (`self.InteractionTransform`))) "Undefined" "MultiplyWithRoot" self "NewEnumerator4" self null))

(event `OnDirectSelected`
  (`GameplayStatics.PlaySound2D` "/Engine/VREditor/Sounds/UI/Click_on_Button.Click_on_Button" 1.0 1.0 0.0 null null))

(event `BasicLerpPos`
  (params (targetLocation :type "Vector Structure"))
  (bind (_direction _alpha) (`Timeline|Timeline` :!via `PlayFromStart` :!label _label_2)
    (:`Update`
      (bind _sweephitresult (`self.K2_SetActorLocation` (`KismetMathLibrary.VLerp` (`self.K2_GetActorLocation`) targetLocation _alpha) true))
      (if (`GameplayStatics.BreakHitResult` _sweephitresult)
        (goto _label_2 :!via `Stop`)))
    (:`Finished`
      (`self.K2_SetActorLocation` targetLocation true))))

(event `Wave Enable`
  (`self.setMeshesEnabled` true))

(event `Wave Disable`
  (`self.setMeshesEnabled` false))

(fn `createHighlightMesh`
  (params (ogMesh :type "MeshComponent Object Reference"))
  (returns (highlightMesh :type "MeshComponent Object Reference"))
  (locals (newHighlightMesh :type "MeshComponent Object Reference") (isStaticMesh :type Boolean) (dynMatInst :type "MaterialInstanceDynamic Object Reference"))
  (bind _returnvalue (`KismetMathLibrary.MakeTransform` (0.0 0.0 0.0)))
  (bind _asskeletal_mesh_component (cast `SkeletalMeshComponent` (`local.ogMesh`) :!pure true))
  (set `local.isStaticMesh` (`.bSuccess` (cast `StaticMeshComponent` ogMesh :!pure true)))
  (`|ExecutionSequence`
    (:`then_0`
      (if (`local.isStaticMesh`)
        (bind _returnvalue_2 (`AddComponent|NODE_AddStaticMeshComponent-1` :`RelativeTransform` _returnvalue))
        (set `local.newHighlightMesh` _returnvalue_2)
        (else
          (bind _returnvalue_3 (`AddComponent|NODE_AddSkeletalMeshComponent-0` :`RelativeTransform` _returnvalue))
          (set `local.newHighlightMesh` _returnvalue_3)))
      (`/Engine/EditorBlueprintResources/StandardMacros.IsValid` (`local.newHighlightMesh`)
        (:`Is Valid`
          (`SceneComponent.K2_AttachToComponent` (`local.newHighlightMesh`) (`local.ogMesh`) "None" "SnapToTarget" "SnapToTarget" "KeepRelative" true)
          (`PrimitiveComponent.SetCollisionEnabled` (`local.newHighlightMesh`) "NoCollision")
          (`PrimitiveComponent.SetCastShadow` (`local.newHighlightMesh`) false)
          (`|ExecutionSequence`
            (:`then_0`
              ;[1 1 1] Cast to Static/Skinned, return if neither
              (if (`local.isStaticMesh`)
                (bind _asstatic_mesh_component (cast `StaticMeshComponent` (`local.newHighlightMesh`))
                  (:`then`
                    (`StaticMeshComponent.SetStaticMesh` _asstatic_mesh_component (`StaticMeshComponent.StaticMesh` (cast `StaticMeshComponent` (`local.ogMesh`) :!pure true))))
                  (:`CastFailed`
                    (bind _asskeletal_mesh_component_2 (cast `SkeletalMeshComponent` (`local.newHighlightMesh`) :!label _label)
                      (:`then`
                        (`SkeletalMeshComponent.SetSkeletalMeshAsset` _asskeletal_mesh_component_2 (`SkeletalMeshComponent.GetSkeletalMeshAsset` _asskeletal_mesh_component))
                        (bind _lastplayedanim (`self.lastPlayedAnim`)
                          (:`then`
                            (`self.playAnimation` _asskeletal_mesh_component _lastplayedanim))
                          (:`else`)))
                      (:`CastFailed`
                        (return null)))))
                (else
                  (goto _label))))
            (:`then_1`
              ;[1 1 1] Setup materials
              (bind _returnvalue_4 (`KismetMaterialLibrary.CreateDynamicMaterialInstance` "/Game/Materials/FXandParticles/M_Outline.M_Outline"))
              (set `local.dynMatInst` _returnvalue_4)
              (`self.scaleOutlineParamForSkMesh` (`local.dynMatInst`) "Thickness" (`local.isStaticMesh`))
              (`self.scaleOutlineParamForSkMesh` (`local.dynMatInst`) "AdditionalBeatThickness" (`local.isStaticMesh`))
              (for (_ _array_index) (`MeshComponent.GetMaterials` (`local.newHighlightMesh`))
                (`PrimitiveComponent.SetMaterial` (`local.newHighlightMesh`) _array_index (`local.dynMatInst`))))))))
    (:`then_1`
      (return (`local.newHighlightMesh`)))))

(fn `drawWaterFrom`
  (returns (liquidGlob :type "/Game/Blueprints/Player/LiquidGlob/BP_LiquidGlob Object Reference"))
  (bind _returnvalue (`|SpawnActorFromClass` "/Game/Blueprints/Player/LiquidGlob/BP_LiquidGlob.BP_LiquidGlob_C" (`KismetMathLibrary.Conv_VectorToTransform` (`self.K2_GetActorLocation`)) "Undefined" "MultiplyWithRoot" (`GameplayStatics.GetPlayerPawn` 0) null))
  (return _returnvalue))

(fn `getCenterOfMass`
  (returns (centerOfMass :type "Vector Structure") (success :type Boolean))
  (locals (mesh :type "MeshComponent Object Reference") (COM :type "Vector Structure" :default (0.0 0.0 0.0)))
  (bind (_mesh _success) (`self.getMainMesh`))
  (bind _mesh_2 (`local.mesh`))
  (bind (_asskeletal_mesh_component _bsuccess) (cast `SkeletalMeshComponent` _mesh_2 :!pure true))
  (bind _output_get (set `local.mesh` _mesh))
  (if _success
    (set `local.COM` (`KismetMathLibrary.SelectVector` (`SkeletalMeshComponent.GetSkeletalCenterOfMass` _asskeletal_mesh_component) (`PrimitiveComponent.GetCenterOfMass` _mesh_2 "None") _bsuccess))
    (`KismetSystemLibrary.PrintString` (`KismetStringLibrary.Concat_StrStr` (`KismetSystemLibrary.GetDisplayName` _output_get) "'s Center of Mass is: " (`KismetStringLibrary.Conv_VectorToString` (`local.COM`))) true true (struct :`R` 1.0 :`G` 0.572535 :`B` 0.338429 :`A` 1.0) 10.0)
    (return (+ (`local.COM`) (`self.K2_GetActorLocation`)) true)
    (else
      (return (0.0 0.0 0.0) false))))

(fn `getCenterOfMassOffset`
  (returns (offset :type "Vector Structure") (success :type Boolean))
  (bind (_centerofmass _success) (`self.getCenterOfMass`))
  (if _success
    (return (- _centerofmass (`self.K2_GetActorLocation`)) true)
    (else
      (return (0.0 0.0 0.0) false))))

(fn `getGrabPhysicsSimulators`
  (returns (physicsSimulators :type "Array of PrimitiveComponent Object Reference"))
  (return (`self.MESHES`)))

(fn `getInteractionTransform`
  (returns (interactionTransform :type "SceneComponent Object Reference"))
  (return (`self.InteractionTransform`)))

(fn `getMainMesh`
  (returns (mesh :type "MeshComponent Object Reference") (success :type Boolean))
  (bind _output (`|GetArrayItem` (`self.MESHES`)))
  (return _output (`KismetSystemLibrary.IsValid` _output)))

(fn `getProperties`
  (returns (properties :type "Array of /Game/Blueprints/Interactive/EInteractiveProperty Enum"))
  (bind _properties (`/Game/Blueprints/Interactive/BPI_Interactive.getProperties` (`self.BPC_Interactive`)))
  (return _properties))

(fn `interactStart`
  (params (caller :type "/Game/Blueprints/Interactive/BPI_Interactive Interface") (interactionType :type "/Game/Blueprints/Interactive/EInteractionType Enum" :default "NewEnumerator0"))
  (returns (electrifiedFX :type "/Game/Blueprints/Player/Electricity/BP_Electrified Object Reference") (isGrabbable :type Boolean))
  (`|ExecutionSequence`
    (:`then_0`
      (if (`|EnumEquality` interactionType "NewEnumerator6")
        (`self.OnDirectSelected`)
        (return null false)))
    (:`then_1`
      (if (`|EnumEquality` interactionType "NewEnumerator7")
        (`self.Wave Enable`)
        (return null false)))
    (:`then_2`
      (bind (_electrifiedfx _isgrabbable) (`/Game/Blueprints/Interactive/BPI_Interactive.interactStart` (`self.BPC_Interactive`) caller interactionType))
      (return _electrifiedfx _isgrabbable))))

(fn `interactStop`
  (params (caller :type "/Game/Blueprints/Interactive/BPI_Interactive Interface") (interactionType :type "/Game/Blueprints/Interactive/EInteractionType Enum" :default "NewEnumerator0"))
  (returns (success :type Boolean))
  (if (`|EnumEquality` interactionType "NewEnumerator7")
    (`self.Wave Disable`)
    (return true)
    (else
      (bind _success (`/Game/Blueprints/Interactive/BPI_Interactive.interactStop` (`self.BPC_Interactive`) caller interactionType))
      (return _success))))

(fn `playAnimation`
  (params (skMesh :type "SkeletalMeshComponent Object Reference") (anim :type "AnimationAsset Object Reference"))
  (set `self.lastPlayedAnim` (cast `AnimSequence` anim :!pure true))
  (`SkeletalMeshComponent.PlayAnimation` skMesh anim true)
  (for _array_element (`SceneComponent.GetChildrenComponents` (`local.skMesh`) false)
    (bind _asskeletal_mesh_component (cast `SkeletalMeshComponent` _array_element))
    (if (== (`SkeletalMeshComponent.GetSkeletalMeshAsset` _asskeletal_mesh_component) (`SkeletalMeshComponent.GetSkeletalMeshAsset` (`local.skMesh`)))
      (`SkeletalMeshComponent.PlayAnimation` _asskeletal_mesh_component (`local.anim`) true))))

(fn `scaleOutlineParamForSkMesh`
  (params (dynMatInst :type "MaterialInstanceDynamic Object Reference") (param :type Name :default "Thickness") (isStaticMesh :type Boolean))
  (bind _returnvalue (`MaterialInstanceDynamic.K2_GetScalarParameterValue` dynMatInst param))
  (`MaterialInstanceDynamic.SetScalarParameterValue` dynMatInst param (`KismetMathLibrary.SelectFloat` _returnvalue (/ _returnvalue 100.0) isStaticMesh)))

(fn `setHighlighted`
  (params (newHighlighted :type Boolean))
  (if (`.success` (`self.getMainMesh`))
    (if (`local.newHighlighted`)
      (`|ExecutionSequence`
        (:`then_0`
          (if (`KismetArrayLibrary.Array_IsEmpty` (`self.highlightMeshes`))
            (for _array_element (`self.MESHES`)
              (bind _highlightmesh (`self.createHighlightMesh` _array_element))
              (`/Engine/EditorBlueprintResources/StandardMacros.IsValid` _highlightmesh
                (:`Is Valid`
                  (`KismetArrayLibrary.Array_Add` (`self.highlightMeshes`) _highlightmesh))))))
        (:`then_1`
          (`self.setHighlightMeshesVisibility` true)))
      (else
        (`self.setHighlightMeshesVisibility` false)))))

(fn `setHighlightMeshesVisibility`
  (params (newVisibility :type Boolean))
  (for _array_element (`self.highlightMeshes`)
    (`SceneComponent.SetVisibility` _array_element newVisibility false)))

(fn `setMaterialScalar`
  (params (ParameterName :type Name) (Value :type "Float (single-precision)"))
  (`self.tryCreateDynamicMaterialsForMeshes`)
  (for _array_element (`self.MESHES`)
    (for _array_element_2 (`MeshComponent.GetMaterials` _array_element)
      (bind _asmaterial_instance_dynamic (cast `MaterialInstanceDynamic` _array_element_2))
      (`MaterialInstanceDynamic.SetScalarParameterValue` _asmaterial_instance_dynamic (`local.ParameterName`) (`local.Value`)))))

(fn `setMeshes`
  (params (inMESHES :type "Array of MeshComponent Object Reference") (addNotSet :type Boolean))
  (`|ExecutionSequence`
    (:`then_0`
      (if addNotSet
        ;[1 1 1] Add more
        (for _array_element (`local.inMESHES`)
          (`KismetArrayLibrary.Array_AddUnique` (`self.MESHES`) _array_element))
        (else
          ;[1 1 1] Direct set
          (set `self.MESHES` (`local.inMESHES`)))))))

(fn `setMeshesEnabled`
  (params (newEnabled :type Boolean))
  (`self.setHighlightMeshesVisibility` newEnabled)
  (`|ExecutionSequence`
    (:`then_0`
      (for _array_element (`self.MESHES`)
        (`SceneComponent.SetVisibility` _array_element (`local.newEnabled`) false)))
    (:`then_1`
      (`self.SetActorEnableCollision` (`local.newEnabled`)))))

(fn `startElectrified`
  (returns (electrifiedFX :type "/Game/Blueprints/Player/Electricity/BP_Electrified Object Reference"))
  (bind (_returnvalue_location _returnvalue_rotation) (`KismetMathLibrary.BreakTransform` (`SceneComponent.K2_GetComponentToWorld` (`self.InteractionTransform`))))
  (bind _returnvalue (`|SpawnActorFromClass` "/Game/Blueprints/Player/Electricity/BP_Electrified.BP_Electrified_C" (`KismetMathLibrary.MakeTransform` _returnvalue_location _returnvalue_rotation) "Undefined" "MultiplyWithRoot" null (`self.InteractionTransform`) self null))
  (bind _output_get (set `self.electrifiedFX` _returnvalue))
  (return _output_get))

(fn `tryCreateDynamicMaterialsForMeshes`
  (if (not (`self.hasDynamicMats`))
    (for (_array_element _array_index) (`self.MESHES`)
      (for _array_element_2 (`MeshComponent.GetMaterials` _array_element)
        (bind _returnvalue (`MaterialInterface.GetBaseMaterial` _array_element_2))
        (if (== _returnvalue "/Game/Materials/_Master/M_Master.M_Master")
          (bind _returnvalue_2 (`KismetMaterialLibrary.CreateDynamicMaterialInstance` _array_element_2))
          (`PrimitiveComponent.SetMaterial` _array_element _array_index _returnvalue_2))))
    (set `self.hasDynamicMats` true)))

(fn `UserConstructionScript`)